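; US laser-designator binoculars that place a LazeTarget actor where the user aims.
; On zoom changes, the authority flips LazeMode and destroys the target when it turns off, while non-authority instances start or pause a looping trace timer.
; While LazeMode is set, each trace runs forward from the first-person mesh's binoculars socket, spawning or moving the target on a hit and removing it on a miss.
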(event `self.BlueprintOnUnequip`
  (set `self.ControllerRef` null))

(event `self.ReceiveTick`
  (params (DeltaSeconds :type "Float (single-precision)"))
  (`parent.ReceiveTick` DeltaSeconds))

(event `self.BlueprintOnEquip`
  (bind _assqsoldier (cast `SQSoldier` (`self.GetOwner` self)))
  (bind _asbp_player_controller (cast `/Game/Blueprints/BP_PlayerController` (`Pawn.GetController` _assqsoldier)))
  (set `self.ControllerRef` _asbp_player_controller))

(event `TraceLazePosition`
  (bind _mesh1p (`self.Mesh1P`))
  (bind _returnvalue (`SceneComponent.GetSocketLocation` _mesh1p "binoculars_base"))
  (if (`self.LazeMode`)
    (bind (_outhit _returnvalue_2) (`KismetSystemLibrary.LineTraceSingle` _returnvalue (+ _returnvalue (* (`KismetMathLibrary.Conv_RotatorToVector` (`SceneComponent.GetSocketRotation` _mesh1p "binoculars_base")) (`KismetMathLibrary.Conv_IntToDouble` (`self.LazeDistance`)))) "TraceTypeQuery1" false (`|MakeArray` self :!type "Actor Object Reference")))
    (if _returnvalue_2
      (`self.UpdateLazePosition` (`.Location` (`GameplayStatics.BreakHitResult` _outhit)))
      (else
        (`self.UpdateLazePosition` (0.0 0.0 0.0) true)))))

(event `UpdateLazePosition`
  (params (NewLocation :type "Vector Structure") (`Delete Laze` :type Boolean))
  (bind _lazepoint (`self.LazePoint`))
  (bind _lazepoint_2 (`self.LazePoint`))
  (if `Delete Laze`
    (`/Engine/EditorBlueprintResources/StandardMacros.IsValid` _lazepoint_2
      (:`Is Valid`
        (`self.K2_DestroyActor` _lazepoint_2))
      (:`Is Not Valid`
        _))
    (set `self.LazePoint` null)
    (else
      (bind _output_get (set `self.LazeLocation` NewLocation))
      (`/Engine/EditorBlueprintResources/StandardMacros.IsValid` _lazepoint
        (:`Is Valid`
          (`self.K2_SetActorLocation` _lazepoint _output_get false false))
        (:`Is Not Valid`
          (bind _returnvalue (`|SpawnActorFromClass` "/HelicopterTestMaps/Soldiers/Binoculars/LazeTarget.LazeTarget_C" (`KismetMathLibrary.MakeTransform` (`self.LazeLocation`)) "Undefined" "OverrideRootScale"))
          (set `self.LazePoint` _returnvalue))))))

(event `self.BlueprintOnZoom`
  (params (bNewZoom :type Boolean))
  (bind _lazepoint (`self.LazePoint`))
  (`/Engine/EditorBlueprintResources/ActorMacros.Switch Has Authority`
    (:`Authority`
      (bind _isa (`/Engine/EditorBlueprintResources/StandardMacros.FlipFlop`)
        (:`A`
          _)
        (:`B`
          _))
      (bind _output_get (set `self.LazeMode` _isa))
      (if (not _output_get)
        (`/Engine/EditorBlueprintResources/StandardMacros.IsValid` _lazepoint
          (:`Is Valid`
            (`self.K2_DestroyActor` _lazepoint)
            (set `self.LazePoint` null)))))
    (:`Remote`
      (if bNewZoom
        (bind _returnvalue (`KismetSystemLibrary.K2_SetTimerDelegate` (delegate `TraceLazePosition`) 0.05 true))
        (else
          (`KismetSystemLibrary.K2_PauseTimerHandle` _returnvalue))))))

(fn `UserConstructionScript`
  (`parent.UserConstructionScript`))