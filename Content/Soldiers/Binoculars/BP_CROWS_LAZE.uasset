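; CROWS laser designator turret seat (Squad vehicle) with clamped yaw and pitch aiming, fire passed to the current vehicle weapon and two-camera zoom toggle.
; NewLaze registers laze target actors, which are dropped again when destroyed.
; While viewed, the local player gets one marker widget per target, projected to screen each Tick.
; Widgets pair with targets by array index, so removal simply pops the last widget.
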(event `InputAxis|Turn`
  (params (AxisValue :type "Float (single-precision)"))
  (bind _maxrotationspeed (`self.MaxRotationSpeed`))
  (`self.AddControllerYawInput` (`KismetMathLibrary.FClamp` (* AxisValue (`self.RotationSpeedMultiplier`)) (* _maxrotationspeed -1.0) _maxrotationspeed)))

(event `InputAxis|LookUp`
  (params (AxisValue :type "Float (single-precision)"))
  (bind (_returnvalue_roll _returnvalue_pitch) (`KismetMathLibrary.BreakRotator` (`self.GetControlRotation`)))
  (bind _pitchlimit (`self.PitchLimit`))
  (bind _maxelevationspeed (`self.MaxElevationSpeed`))
  (bind _minpitchlimit (`self.MinPitchLimit`))
  (bind _returnvalue (* (select `bool` (>= _returnvalue_pitch 180.0) :`false` _returnvalue_pitch :`true` (- _returnvalue_pitch 360.0)) -1.0))
  (`self.AddControllerPitchInput` (`KismetMathLibrary.FClamp` (`KismetMathLibrary.FClamp` (* AxisValue (`self.ElevationSpeedMultiplier`)) (* _maxelevationspeed -1.0) _maxelevationspeed) (`KismetMathLibrary.FClamp` (- _minpitchlimit _returnvalue) _minpitchlimit 0.0) (`KismetMathLibrary.FClamp` (- _pitchlimit _returnvalue) 0.0 _pitchlimit))))

(event `self.K2_OnBecomeViewTarget`
  (params (PC :type "PlayerController Object Reference"))
  (for _ (`self.LazeTarget`)
    (bind _returnvalue (`|CreateWidget` "/HelicopterTestMaps/Soldiers/Binoculars/LazeMarkerWidget.LazeMarkerWidget_C" PC))
    (`KismetArrayLibrary.Array_Add` (`self.LazeWidget`) _returnvalue)
    (`UserWidget.AddToViewport` _returnvalue 0))
  (set `self.CameraEnabled` true))

(event `self.K2_OnEndViewTarget`
  (params (PC :type "PlayerController Object Reference"))
  (bind _lazewidget (`self.LazeWidget`))
  (set `self.CameraEnabled` false)
  (for _array_element _lazewidget
    (`Widget.RemoveFromParent` _array_element))
  (`KismetArrayLibrary.Array_Clear` _lazewidget))

(event `InputAction|Fire`
  (params (Key :type "Key Structure" :default "AnyKey"))
  (bind _currentweapon (`SQPawnInventoryComponent.CurrentWeapon` (`self.GetVehicleInventory`)))
  (:`Pressed`
    (`SQEquipableItem.BeginUse` _currentweapon))
  (:`Released`
    (`SQEquipableItem.EndUse` _currentweapon)))

(event `New Laze`
  (params (`Laze Actor` :type "/HelicopterTestMaps/Soldiers/Binoculars/LazeTarget Object Reference"))
  (`KismetSystemLibrary.PrintString` "New Laze msg")
  (`KismetArrayLibrary.Array_Add` (`self.LazeTarget`) `Laze Actor`)
  (add `self.OnDestroyed` `Laze Actor` (delegate `RemoveLazeActor`))
  (if (`self.IsLocallyControlled` self)
    (if (`self.CameraEnabled`)
      (bind _asplayer_controller (cast `PlayerController` (`self.GetController` self)))
      (bind _returnvalue (`|CreateWidget` "/HelicopterTestMaps/Soldiers/Binoculars/LazeMarkerWidget.LazeMarkerWidget_C" _asplayer_controller))
      (`/Engine/EditorBlueprintResources/StandardMacros.IsValid` _returnvalue
        (:`Is Valid`
          (`Widget.SetRenderTranslation` _returnvalue (-32.0 -32.0))
          (bind _returnvalue_2 (`KismetArrayLibrary.Array_Add` (`self.LazeWidget`) _returnvalue))
          (`UserWidget.AddToViewport` _returnvalue 0)
          (`KismetSystemLibrary.PrintString` (`KismetStringLibrary.Conv_IntToString` _returnvalue_2)))))))

(event `RemoveLazeActor` :!signature `self.OnDestroyed`
  (params (DestroyedActor :type "Actor Object Reference"))
  (bind _lazewidget (`self.LazeWidget`))
  (bind _returnvalue (`KismetArrayLibrary.Array_LastIndex` _lazewidget))
  (bind _aslaze_target (cast `/HelicopterTestMaps/Soldiers/Binoculars/LazeTarget` DestroyedActor))
  (`KismetArrayLibrary.Array_RemoveItem` (`self.LazeTarget`) _aslaze_target)
  (if (`self.IsLocallyControlled` self)
    (`Widget.RemoveFromParent` (`|GetArrayItem` _lazewidget _returnvalue))
    (`KismetArrayLibrary.Array_Remove` _lazewidget _returnvalue)))

(event `self.ReceiveBeginPlay`
  (set `SQStaticTurretMovementComponent.YawComponent` (`self.DefaultSceneRoot`) (`self.SQStaticTurretMovement`))
  (set `SQStaticTurretMovementComponent.PitchComponent` (`self.GunAttachPoint`) (`self.SQStaticTurretMovement`))
  (`ActorComponent.SetActive` (`self.Camera`) true false))

(event `InputAction|VehicleZoom`
  (params (Key :type "Key Structure" :default "AnyKey"))
  ;[1 1 1] Zoom via middle mouse button
  (:`Pressed`
    (`/Engine/EditorBlueprintResources/StandardMacros.FlipFlop`
      (:`A`
        (`ActorComponent.SetActive` (`self.Camera`) false false)
        (`ActorComponent.SetActive` (`self.camerazoom`) true false)
        (`GameplayStatics.PlaySound2D` "/Game/Vehicles/BTR80/Sounds/Turret/Zoom/RU_turret_zoom_out_Cue.RU_turret_zoom_out_Cue"))
      (:`B`
        (`ActorComponent.SetActive` (`self.camerazoom`) false false)
        (`ActorComponent.SetActive` (`self.Camera`) true false)
        (`GameplayStatics.PlaySound2D` "/Game/Vehicles/BTR80/Sounds/Turret/Zoom/RU_turret_zoom_in_Cue.RU_turret_zoom_in_Cue")))))

(event `self.ReceiveTick`
  (params (DeltaSeconds :type "Float (single-precision)"))
  (if (`self.IsLocallyControlled` self)
    (if (`self.CameraEnabled`)
      (bind _asplayer_controller (cast `PlayerController` (`self.GetController` self)))
      (for (_array_element _array_index) (`self.LazeTarget`)
        (bind _output (`|GetArrayItem` (`self.LazeWidget`) _array_index))
        (`/Engine/EditorBlueprintResources/StandardMacros.IsValid` _output
          (:`Is Valid`
            (`UserWidget.SetPositionInViewport` _output (`GameplayStatics.ProjectWorldToScreen` _asplayer_controller (`self.K2_GetActorLocation` _array_element)) true)))))))

(fn `Get1PAttachComponent`
  (returns (ReturnValue :type "SceneComponent Object Reference"))
  (return (`self.GunAttachPoint`)))

(fn `Get3PAttachComponent`
  (returns (ReturnValue :type "SceneComponent Object Reference"))
  (return (`self.GunAttachPoint`)))

(fn `GetMasterPoseComponent`
  (returns (ReturnValue :type "SkinnedMeshComponent Object Reference"))
  (return null))

(fn `GetSoldierAttachComponent`
  (returns (ReturnValue :type "SceneComponent Object Reference"))
  (return (`SQVehicle.VehicleMesh` (`self.GetVehicle`))))

(fn `GetWeaponAttachComponent`
  (returns (ReturnValue :type "SceneComponent Object Reference"))
  (return (`self.GunAttachPoint`)))

(fn `UserConstructionScript`)