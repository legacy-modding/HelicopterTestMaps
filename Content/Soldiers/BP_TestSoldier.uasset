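; BP_TestSoldier is a test soldier Blueprint that prototypes picking up or dragging another soldier with the Interact key.
; When not falling, flying or sprinting, a camera sphere trace finds a soldier on the same team, without any injury check despite the IsHurt name.
; ServerAttach then unragdolls that soldier, disables mesh physics and snaps actor and mesh onto the player.
; A physics-handle drag variant updated on Tick remains, but its MultiAttach call never runs.
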(event `InputAction|Interact` :overrideparent false
  (params (Key :type "Key Structure" :default "AnyKey"))
  (:`Pressed`
    (bind _allowdrag (`self.MovementBlock`))
    (if _allowdrag
      (bind (_is_hurt _othersoldier) (`self.CanPickupSoldier`))
      (if _is_hurt
        (`self.PickupDrag` _is_hurt _othersoldier)))))

(event `PickupDrag`
  (params (CanDrag :type Boolean) (Soldier :type "SQSoldier Object Reference"))
  (if CanDrag
    (if (`KismetSystemLibrary.IsValid` Soldier)
      (`KismetSystemLibrary.Delay` 0.01)
      (`KismetSystemLibrary.PrintString` (`KismetSystemLibrary.GetDisplayName` Soldier))
      (`self.ServerAttach` Soldier (+ (`SceneComponent.K2_GetComponentLocation` (`self.CapsuleComponent`)) (0.0 0.0 5.0)) self))))

(event `ServerAttach`
  (params (Soldier :type "SQSoldier Object Reference") (Location :type "Vector Structure") (Parent :type "SQSoldier Object Reference"))
  (bind _mesh (`Character.Mesh` Soldier))
  (bind _mesh_2 (`Character.Mesh` Soldier))
  (`SQSoldierRagdollComponent.UnragdollSoldier` (`SQSoldier.RagdollComponent` Soldier) false)
  (`PrimitiveComponent.SetEnableGravity` _mesh_2 false)
  (`PrimitiveComponent.SetEnableGravity` (`Character.CapsuleComponent` Soldier) false)
  (`PrimitiveComponent.SetCollisionEnabled` _mesh_2 "PhysicsOnly")
  (`PrimitiveComponent.SetSimulatePhysics` _mesh_2 false)
  (`SceneComponent.K2_SetRelativeLocation` _mesh (0.0 0.0 0.0) false true)
  (`self.K2_AttachToActor` Soldier Parent "None" "SnapToTarget" "SnapToTarget" "KeepRelative" false)
  (`SceneComponent.K2_AttachToComponent` _mesh (`self.K2_GetRootComponent` Parent) "None" "SnapToTarget" "SnapToTarget" "KeepRelative" false))

(event `self.ReceiveTick`
  (params (DeltaSeconds :type "Float (single-precision)"))
  (bind _body_drag_handle (`self.Body Drag Handle`))
  (bind (_returnvalue_location _returnvalue_rotation) (`KismetMathLibrary.BreakTransform` (`SceneComponent.GetSocketTransform` (`self.Mesh1P`) "SKS_Throw_Particle" "RTS_World")))
  (`/Engine/EditorBlueprintResources/StandardMacros.IsValid` _body_drag_handle
    (:`Is Valid`
      (`PhysicsHandleComponent.SetTargetLocationAndRotation` _body_drag_handle _returnvalue_location _returnvalue_rotation))))

(event `Multi Attach`
  (params (Soldier :type "SQSoldier Object Reference") (Location :type "Vector Structure") (Parent :type "SQSoldier Object Reference"))
  (bind _mesh (`Character.Mesh` Soldier))
  (`SQSoldierRagdollComponent.UnragdollSoldier` (`SQSoldier.RagdollComponent` Soldier) false)
  (`PrimitiveComponent.SetSimulatePhysics` (`Character.Mesh` Soldier) true)
  (`SceneComponent.K2_SetRelativeLocation` _mesh (0.0 0.0 0.0) false true)
  (bind _returnvalue (`AddComponent|NODE_AddPhysicsHandleComponent-3`))
  (bind _output_get (set `self.Body Drag Handle` _returnvalue))
  (`PhysicsHandleComponent.GrabComponentAtLocation` _output_get _mesh "None" Location))

(fn `CanPickupSoldier`
  (returns (`Is hurt` :type Boolean) (OtherSoldier :type "SQSoldier Object Reference"))
  (bind _returnvalue (`SceneComponent.GetSocketLocation` (`self.Mesh`) "CameraSocket"))
  (bind (_outhit _returnvalue_2) (`KismetSystemLibrary.SphereTraceSingleForObjects` _returnvalue (+ _returnvalue (* (`KismetMathLibrary.Conv_RotatorToVector` (`.OutRotation` (`self.GetActorEyesViewPoint`))) (`KismetMathLibrary.Conv_IntToDouble` 100))) 35.0 (`self.Interact Object Types`) false (`|MakeArray` self :!type "Actor Object Reference")))
  (if _returnvalue_2
    (bind (_bblockinghit _binitialoverlap _time _location _impactpoint _normal _impactnormal _physmat _hitactor) (`GameplayStatics.BreakHitResult` _outhit))
    (if (`KismetSystemLibrary.IsValid` _hitactor)
      (bind _assqsoldier (cast `SQSoldier` _hitactor)
        (:`then`
          (bind _assqplayer_state (cast `SQPlayerState` (`self.PlayerState`))
            (:`then`
              ;[1 1 1] Other Person's state
              (bind _assqplayer_state_2 (cast `SQPlayerState` (`Pawn.PlayerState` _assqsoldier))
                (:`then`
                  (if (== (`SQTeamState.Id` (`SQPlayerState.TeamState` _assqplayer_state_2)) (`SQTeamState.Id` (`SQPlayerState.TeamState` _assqplayer_state)))
                    (return true _assqsoldier)
                    (else
                      _)))
                (:`CastFailed`
                  _)))
            (:`CastFailed`
              _)))
        (:`CastFailed`
          _))))
  (return false null))

(fn `MovementBlock`
  (returns (AllowDrag :type Boolean))
  (bind _assqsoldier (cast `SQSoldier` (`self.GetOwner`))
    (:`then`
      (bind _assqsoldier_movement (cast `SQSoldierMovement` (`self.GetMovementComponent` _assqsoldier))
        (:`then`
          _)
        (:`CastFailed`
          _)))
    (:`CastFailed`
      _))
  (return (not (or (`NavMovementComponent.IsFalling` _assqsoldier_movement) (`NavMovementComponent.IsFlying` _assqsoldier_movement) (`SQSoldierMovement.IsSprinting` _assqsoldier_movement)))))

(fn `UserConstructionScript`
  (`parent.UserConstructionScript`))