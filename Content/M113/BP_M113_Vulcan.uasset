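; Tracked vehicle Blueprint for the M113 Vulcan, handling driver cameras and animated track visuals.
; The driver camera turns within yaw and pitch limits, and a zoom input toggles an orbiting spring-arm external camera when world settings allow third person.
; Construction creates dynamic materials for both tracks, and cosmetic-only Tick scrolls their texture offsets from each track's speed in the movement component.
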(event `self.ReceiveBeginPlay`
  ;[1 1 1] Camera Setup
  (`ActorComponent.Activate` (`self.Camera`) false)
  (`ActorComponent.Deactivate` (`self.ExternalCamera`)))

(event `InputAction|VehicleZoom`
  (params (Key :type "Key Structure" :default "AnyKey"))
  (bind _externalcamera (`self.ExternalCamera`))
  (bind _camera (`self.Camera`))
  ;[1 1 1] Third Person Debug Camera
  (:`Pressed`
    (bind _returnvalue (`SQBlueprintLibrary.GetWorldSettings`))
    (bind _assqworld_settings (cast `SQWorldSettings` _returnvalue))
    (if (`SQWorldSettings.bCanDriverSwitchTo3rdPerson` _assqworld_settings)
      (if (`ActorComponent.IsActive` (`self.Camera`))
        (`ActorComponent.Deactivate` _camera)
        (`ActorComponent.Activate` _externalcamera false)
        (else
          (`ActorComponent.Activate` _camera false)
          (`ActorComponent.Deactivate` _externalcamera))))))

(event `Key|MouseScrollUp`
  (params (Key :type "Key Structure" :default "AnyKey"))
  (bind _springarm (`self.SpringArm`))
  ;[1 1 1] Third Person Debug Camera
  (:`Pressed`
    (if (`ActorComponent.IsActive` (`self.ExternalCamera`))
      (set `SpringArmComponent.TargetArmLength` (`KismetMathLibrary.FMax` (- (`SpringArmComponent.TargetArmLength` _springarm) 250.0)) _springarm))))

(event `Key|MouseScrollDown`
  (params (Key :type "Key Structure" :default "AnyKey"))
  (bind _springarm (`self.SpringArm`))
  ;[1 1 1] Third Person Debug Camera
  (:`Pressed`
    (if (`ActorComponent.IsActive` (`self.ExternalCamera`))
      (set `SpringArmComponent.TargetArmLength` (+ (`SpringArmComponent.TargetArmLength` _springarm) 250.0) _springarm))))

(event `InputAxisKey|MouseX`
  (params (AxisValue :type "Float (single-precision)"))
  ;[1 1 1] Third Person Debug Camera
  (if (`ActorComponent.IsActive` (`self.ExternalCamera`))
    (`SceneComponent.K2_AddLocalRotation` (`self.SpringArm`) (`KismetMathLibrary.MakeRotator` 0.0 0.0 AxisValue) false false)))

(event `InputAxisKey|MouseY`
  (params (AxisValue :type "Float (single-precision)"))
  ;[1 1 1] Third Person Debug Camera
  (if (`ActorComponent.IsActive` (`self.ExternalCamera`))
    (`SceneComponent.K2_AddLocalRotation` (`self.SpringArm`) (`KismetMathLibrary.MakeRotator` 0.0 AxisValue) false false)))

(event `InputAxis|Turn`
  (params (AxisValue :type "Float (single-precision)"))
  (bind _yawlimit (`self.YawLimit`))
  (bind _returnvalue (* _yawlimit -1.0))
  (bind (_relativerotation_roll _relativerotation_pitch _relativerotation_yaw) (`KismetMathLibrary.BreakRotator` (`SceneComponent.RelativeRotation` (`self.Camera`))))
  (bind _returnvalue_2 (select `bool` (>= _relativerotation_yaw 180.0) :`false` _relativerotation_yaw :`true` (- _relativerotation_yaw 360.0)))
  (`SceneComponent.K2_AddRelativeRotation` (`self.Camera`) (`KismetMathLibrary.MakeRotator` 0.0 0.0 (`KismetMathLibrary.FClamp` AxisValue (`KismetMathLibrary.FClamp` (- _returnvalue _returnvalue_2) _returnvalue 0.0) (`KismetMathLibrary.FClamp` (- _yawlimit _returnvalue_2) 0.0 _yawlimit))) false false))

(event `InputAxis|LookUp`
  (params (AxisValue :type "Float (single-precision)"))
  (bind _pitchlimit (`self.PitchLimit`))
  (bind _returnvalue (* (`self.PitchLimit`) -1.0))
  (bind (_relativerotation_roll _relativerotation_pitch) (`KismetMathLibrary.BreakRotator` (`SceneComponent.RelativeRotation` (`self.Camera`))))
  (bind _returnvalue_2 (select `bool` (>= _relativerotation_pitch 180.0) :`false` _relativerotation_pitch :`true` (- _relativerotation_pitch 360.0)))
  ;[1 1 1] Driver Head Rotation
  (`SceneComponent.K2_AddRelativeRotation` (`self.Camera`) (`KismetMathLibrary.MakeRotator` 0.0 (`KismetMathLibrary.FClamp` (* AxisValue -1.0) (`KismetMathLibrary.FClamp` (- _returnvalue _returnvalue_2) _returnvalue 0.0) (`KismetMathLibrary.FClamp` (- _pitchlimit _returnvalue_2) 0.0 _pitchlimit))) false false))

(event `self.ReceiveTick`
  (params (DeltaSeconds :type "Float (single-precision)"))
  (`parent.ReceiveTick` DeltaSeconds)
  (`/Engine/EditorBlueprintResources/StandardMacros.Can Execute Cosmetic Events`
    (:`True`
      (bind _assqtracked_vehicle_movement_component (cast `SQTrackedVehicleMovementComponent` (`self.VehicleMovement`)))
      (`|ExecutionSequence`
        (:`then_0`
          (bind _newuvoffset (`self.UpdateTrackMaterial` DeltaSeconds (`WheeledVehicleMovementComponentTank.GetRightTrackSpeed` _assqtracked_vehicle_movement_component) (`self.TrackMaterialRight`) (`self.RightTrackUVOffset`)))
          (set `self.RightTrackUVOffset` _newuvoffset))
        (:`then_1`
          (bind _newuvoffset_2 (`self.UpdateTrackMaterial` DeltaSeconds (`WheeledVehicleMovementComponentTank.GetLeftTrackSpeed` _assqtracked_vehicle_movement_component) (`self.TrackMaterialLeft`) (`self.LeftTrackUVOffset`)))
          (set `self.LeftTrackUVOffset` _newuvoffset_2))))))

(fn `UpdateTrackMaterial`
  (params (DeltaTime :type "Float (double-precision)") (MovementSpeed :type "Float (double-precision)") (TrackMaterial :type "MaterialInstanceDynamic Object Reference") (TrackOffset :type "Float (double-precision)"))
  (returns (NewUVOffset :type "Float (double-precision)"))
  (bind _returnvalue (mod (+ (* DeltaTime (/ (/ (- 0.0 MovementSpeed) 200.0) 2.0)) TrackOffset) 1.0))
  (`/Engine/EditorBlueprintResources/StandardMacros.IsValid` TrackMaterial
    (:`Is Valid`
      (if (> (`KismetMathLibrary.Abs` MovementSpeed) 0.1)
        (`MaterialInstanceDynamic.SetScalarParameterValue` TrackMaterial "CurrentOffset" _returnvalue)
        (return _returnvalue)
        (else
          _)))
    (:`Is Not Valid`
      _))
  (return TrackOffset))

(fn `UserConstructionScript`
  (bind _vehiclemesh (`self.VehicleMesh`))
  (bind _vehiclemesh_2 (`self.VehicleMesh`))
  (bind _returnvalue (`MeshComponent.GetMaterialIndex` _vehiclemesh_2 "track_right"))
  (bind _returnvalue_2 (`MeshComponent.GetMaterialIndex` _vehiclemesh "track_left"))
  (if (`KismetArrayLibrary.Array_IsValidIndex` (`MeshComponent.GetMaterials` _vehiclemesh_2) _returnvalue)
    (bind _returnvalue_3 (`PrimitiveComponent.CreateDynamicMaterialInstance` _vehiclemesh_2 _returnvalue null))
    (set `self.TrackMaterialRight` _returnvalue_3)
    (if (`KismetArrayLibrary.Array_IsValidIndex` (`MeshComponent.GetMaterials` _vehiclemesh) _returnvalue_2)
      (bind _returnvalue_4 (`PrimitiveComponent.CreateDynamicMaterialInstance` _vehiclemesh _returnvalue_2 null))
      (set `self.TrackMaterialLeft` _returnvalue_4))))