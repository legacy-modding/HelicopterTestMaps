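; Helicopter vehicle Blueprint that passes clamped mouse input to the HeliFM flight model as pitch and roll, paused while free-look is held.
; The zoom key toggles InvertControls, which switches horizontal mouse from roll to negated yaw.
; Hard mesh impacts apply damage scaled by impulse.
; Helper logic spins both rotors by engine speed and shows rotor dust at low altitude when engine speed is high enough.
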(event `InputAxis|LookUp`
  (params (AxisValue :type "Float (single-precision)"))
  (bind _pitch_max_speed (`self.Pitch Max Speed`))
  (if (`ActorComponent.IsActive` (`self.ExternalCamera`))
    _
    (else
      _))
  (if (not (`self.Free Looking`))
    (if (`self.InvertControls`)
      _
      (else
        _))
    (`/HelicopterTestMaps/HeliFM.InputControls` (`self.HeliFM`) 1 false (`KismetMathLibrary.FClamp` (* AxisValue (`self.Pitch Speed`)) (* _pitch_max_speed -1.0) _pitch_max_speed) false)))

(event `InputAxisKey|MouseX`
  (params (AxisValue :type "Float (single-precision)"))
  (bind _helifm (`self.HeliFM`))
  (bind _roll_max_speed (`self.Roll Max speed`))
  (bind _returnvalue (+ (`self.Roll Max speed`) 0.3))
  (if (`ActorComponent.IsActive` (`self.ExternalCamera`))
    _
    (else
      _))
  (if (`self.Free Looking`)
    _
    (elif (`self.InvertControls`)
      (`/HelicopterTestMaps/HeliFM.InputControls` _helifm 3 false (* (`KismetMathLibrary.FClamp` (* AxisValue (`self.Mouse Yaw Mul`)) (* _returnvalue -1.0) _returnvalue) -1.0) false)
      (else
        (`/HelicopterTestMaps/HeliFM.InputControls` _helifm 2 false (`KismetMathLibrary.FClamp` (* AxisValue (`self.Roll Speed`)) (* _roll_max_speed -1.0) _roll_max_speed) false)))))

(event `InputAction|FreeLook`
  (params (Key :type "Key Structure" :default "AnyKey"))
  (:`Pressed`
    (set `self.Free Looking` true :!label _label))
  (:`Released`
    (set `self.Free Looking` false :!label _label_2)))

(event `SpawnDust`
  (bind _smokeparticle (`self.SmokeParticle`))
  (bind _helifm (`self.HeliFM`))
  (bind _returnvalue (`KismetMathLibrary.Abs` (`self.Altitude`)))
  (if (> (`/HelicopterTestMaps/HeliFM.Engine Speed` _helifm) (+ (`/HelicopterTestMaps/HeliFM.AntiGravitySpeed` _helifm) -50.0))
    (if (< _returnvalue 1500.0)
      (if (> _returnvalue 0.0)
        (`SceneComponent.SetVisibility` _smokeparticle true false)
        (`SceneComponent.K2_SetWorldTransform` _smokeparticle (`self.DustTransform`) false true)
        (else
          (`SceneComponent.SetVisibility` _smokeparticle false false :!label _label_3)))
      (else
        (goto _label_3)))
    (else
      (goto _label_3))))

(event `InputAction|Crouch`
  (params (Key :type "Key Structure" :default "AnyKey"))
  (:`Pressed`
    (goto _label))
  (:`Released`
    (goto _label_2)))

(event `ServerToggleFiremode`
  (params (Bool :type Boolean))
  (set `self.InvertControls` (not (`self.InvertControls`))))

(event `InputAction|VehicleZoom`
  (params (Key :type "Key Structure" :default "AnyKey"))
  (:`Pressed`
    (`self.ServerToggleFiremode` (not (`self.InvertControls`)))))

(event `self.VehicleMesh.OnComponentHit`
  (params (HitComponent :type "PrimitiveComponent Object Reference") (OtherActor :type "Actor Object Reference") (OtherComp :type "PrimitiveComponent Object Reference") (NormalImpulse :type "Vector Structure") (Hit :type "HitResult Structure (by ref)"))
  (bind _returnvalue (`KismetMathLibrary.VSize` NormalImpulse))
  (if (> _returnvalue (`self.minImpactSpeed`))
    (`GameplayStatics.ApplyDamage` self (* 100 (/ _returnvalue (`self.minImpactSpeed`))) null null "/Script/Squad.SQBurningDamage")
    (set `self.bCanBeDamaged` true)))

(event `MountPlayer`
  (params (Controller :type "SQPlayerController Object Reference"))
  (`SQUsable.ServerOnUsed` Controller))

(fn `SpinRotor`
  (params (EngineSpeed :type "Float (double-precision)"))
  (bind _returnvalue (* EngineSpeed 0.1))
  (`SceneComponent.K2_AddLocalRotation` (`self.RotorMain`) (`KismetMathLibrary.MakeRotator` 0.0 0.0 _returnvalue) false false)
  (`SceneComponent.K2_AddLocalRotation` (`self.RotorTail`) (`KismetMathLibrary.MakeRotator` 0.0 _returnvalue) false false))

(fn `UserConstructionScript`
  (`parent.UserConstructionScript`))