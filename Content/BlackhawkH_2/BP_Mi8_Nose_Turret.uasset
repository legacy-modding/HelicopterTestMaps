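; Mi-8 helicopter nose turret Blueprint that turns player look input into aim limited to the turret's range of travel.
; LookUp, active only while current weapon input is enabled, clamps pitch between separate up and down limits.
; Turn, which skips that check, clamps yaw to a symmetric limit that YawCurve derives from current pitch.
; LookUp also nudges yaw back toward center whenever it exceeds that pitch-dependent limit.
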(event `InputAxis|LookUp`
  (params (AxisValue :type "Float (single-precision)"))
  (bind (_returnvalue_roll _returnvalue_pitch) (`KismetMathLibrary.BreakRotator` (`self.GetControlRotation`)))
  (bind (_returnvalue_roll_2 _returnvalue_pitch_2 _returnvalue_yaw) (`KismetMathLibrary.BreakRotator` (`self.GetControlRotation`)))
  (bind (_returnvalue_roll_3 _returnvalue_pitch_3) (`KismetMathLibrary.BreakRotator` (`self.GetControlRotation`)))
  (bind _pitchlimit (`self.PitchLimit`))
  (bind _returnvalue (* (`self.PitchUpLimit`) -1.0))
  (bind _returnvalue_2 (select `bool` (>= _returnvalue_yaw 180.0) :`false` _returnvalue_yaw :`true` (- _returnvalue_yaw 360.0)))
  (bind _returnvalue_3 (* (select `bool` (>= _returnvalue_pitch_3 180.0) :`false` _returnvalue_pitch_3 :`true` (- _returnvalue_pitch_3 360.0)) -1.0))
  (bind _binputenabled (`self.IsCurrentWeaponInputEnabled`))
  (if _binputenabled
    (`self.AddControllerPitchInput` (`KismetMathLibrary.FClamp` AxisValue (`KismetMathLibrary.FClamp` (- _returnvalue _returnvalue_3) _returnvalue 0.0) (`KismetMathLibrary.FClamp` (- _pitchlimit _returnvalue_3) 0.0 _pitchlimit)))
    (if (> (`KismetMathLibrary.Abs` _returnvalue_2) (`CurveFloat.GetFloatValue` (`self.YawCurve`) (select `bool` (>= _returnvalue_pitch 180.0) :`false` _returnvalue_pitch :`true` (- _returnvalue_pitch 360.0))))
      (`self.AddControllerYawInput` (* 0.1 (* (`KismetMathLibrary.SignOfFloat` _returnvalue_2) -1.0))))))

(event `InputAxis|Turn`
  (params (AxisValue :type "Float (single-precision)"))
  (bind (_returnvalue_roll _returnvalue_pitch) (`KismetMathLibrary.BreakRotator` (`self.GetControlRotation`)))
  (bind (_returnvalue_roll_2 _returnvalue_pitch_2 _returnvalue_yaw) (`KismetMathLibrary.BreakRotator` (`self.GetControlRotation`)))
  (bind _returnvalue (select `bool` (>= _returnvalue_yaw 180.0) :`false` _returnvalue_yaw :`true` (- _returnvalue_yaw 360.0)))
  (bind _returnvalue_2 (`CurveFloat.GetFloatValue` (`self.YawCurve`) (select `bool` (>= _returnvalue_pitch 180.0) :`false` _returnvalue_pitch :`true` (- _returnvalue_pitch 360.0))))
  (bind _returnvalue_3 (* _returnvalue_2 -1.0))
  (`self.AddControllerYawInput` (`KismetMathLibrary.FClamp` AxisValue (`KismetMathLibrary.FClamp` (- _returnvalue_3 _returnvalue) _returnvalue_3 0.0) (`KismetMathLibrary.FClamp` (- _returnvalue_2 _returnvalue) 0.0 _returnvalue_2))))

(fn `UserConstructionScript`
  (`parent.UserConstructionScript`))