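; Pilotable Blackhawk helicopter vehicle with two deployable fastropes that exiting soldiers can be mounted onto.
; Gamepad and keyboard inputs feed the HeliFM flight component, with keyboard throttle ramped gradually while hovering and engine toggle starting or stopping it.
; Tick line-traces altitude for the cockpit screen's flight data and, on destruction, breaks the ropes and spawns a temporary wreck inheriting velocity.
; Also handles clamped pilot free-look and a non-shipping external camera toggle.
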(event `InputAxisKey|Gamepad_RightTriggerAxis`
  (params (AxisValue :type "Float (single-precision)"))
  (if (> AxisValue 0.0)
    (set `self.AxisLR` false)
    (if (not false)
      (`/Engine/EditorBlueprintResources/ActorMacros.Switch Has Authority`
        (:`Remote`
          (`/HelicopterTestMaps/HeliFM.InputControls` (`self.HeliFM`) 3 true AxisValue false))))))

(event `InputAxisKey|Gamepad_LeftTriggerAxis`
  (params (AxisValue :type "Float (single-precision)"))
  (if (> AxisValue 0.0)
    (set `self.AxisLR` true))
  (if (`self.IsUsingGamepad`)
    (if (`self.AxisLR`)
      (`/Engine/EditorBlueprintResources/ActorMacros.Switch Has Authority`
        (:`Remote`
          (`/HelicopterTestMaps/HeliFM.InputControls` (`self.HeliFM`) 3 false AxisValue false))))))

(event `Key|AnyKey`
  (params (Key :type "Key Structure" :default "AnyKey"))
  (:`Pressed`
    (if (`KismetInputLibrary.Key_IsGamepadKey` Key)
      (bind _output_get (set `self.IsUsingGamepad` true))
      (`self.ServerSetGamepad` _output_get))))

(event `ServerSetDestroyed`
  (params (Float :type Boolean))
  (set `self.DestroyedWatcher` Float))

(event `InputAxisKey|Gamepad_LeftY`
  (params (AxisValue :type "Float (single-precision)"))
  (if (`self.IsUsingGamepad`)
    (`/Engine/EditorBlueprintResources/ActorMacros.Switch Has Authority`
      (:`Remote`
        (`/HelicopterTestMaps/HeliFM.InputControls` (`self.HeliFM`) 0 false AxisValue false)))))

(event `InputAxisKey|Gamepad_RightY`
  (params (AxisValue :type "Float (single-precision)"))
  (if (`self.IsUsingGamepad`)
    (`/Engine/EditorBlueprintResources/ActorMacros.Switch Has Authority`
      (:`Remote`
        (`/HelicopterTestMaps/HeliFM.InputControls` (`self.HeliFM`) 1 false (* AxisValue 0.3) false)))))

(event `ServerSetGamepad`
  (params (Bool :type Boolean))
  (set `self.IsUsingGamepad` Bool))

(event `ServerSetFloatParam`
  (params (Float :type "Float (double-precision)"))
  (`AudioComponent.SetFloatParameter` (`self.EngineRPMAC`) "EngineSpeed" Float))

(event `InputAxisKey|Gamepad_RightX`
  (params (AxisValue :type "Float (single-precision)"))
  (if (`self.IsUsingGamepad`)
    (`/Engine/EditorBlueprintResources/ActorMacros.Switch Has Authority`
      (:`Remote`
        (`/HelicopterTestMaps/HeliFM.InputControls` (`self.HeliFM`) 2 false (* AxisValue 0.3) false)))))

(event `ServerIncEngine`
  (params (Int :type "Float (double-precision)") (Min :type "Float (double-precision)") (Bypass :type Boolean))
  (`self.IncEngine` Int Min Bypass))

(event `ServerSetHover`
  (params (NewParam :type Integer))
  (set `self.engineHover` NewParam))

(event `ServerSetWarmup`
  (params (NewParam :type Boolean))
  (set `self.warmedUp` NewParam)
  (`SceneComponent.SetVisibility` (`self.ParticleSystem1`) NewParam false)
  (`SceneComponent.SetVisibility` (`self.ParticleSystem_0`) NewParam false))

(event `Key|S`
  (params (Key :type "Key Structure" :default "AnyKey"))
  (:`Pressed`
    (`self.ServerSetS` true)
    (set `self.IsKeyAdjusting` (stale `ServerSetS` Bool) :!label _label)
    (set `self.ThrottleDirection` -1)
    (set `self.IsUsingGamepad` false))
  (:`Released`
    (`self.ServerSetS` false)))

(event `ServerSetS`
  (params (Bool :type Boolean))
  (goto _label))

(event `ServerSetControls`
  (params (Control :type Integer) (Bool :type Boolean))
  (switch `int` Control
    (:`Default`
      (set `self.EngineForward` Bool :!label _label_2))
    (:`0`
      (set `self.isDescending` Bool))
    (:`1`
      (set `self.turnRight` Bool))
    (:`2`
      (set `self.turnLeft` Bool))
    (:`3`
      (goto _label_2))))

(event `Key|D`
  (params (Key :type "Key Structure" :default "AnyKey"))
  (bind _helifm (`self.HeliFM`))
  (bind _returnvalue (`KismetMathLibrary.Conv_BoolToInt` (`self.InvertControls`)))
  (bind _returnvalue_2 (- 3 _returnvalue))
  (:`Pressed`
    (`/Engine/EditorBlueprintResources/ActorMacros.Switch Has Authority`
      (:`Authority`
        _)
      (:`Remote`
        _))
    (`/HelicopterTestMaps/HeliFM.InputControls` _helifm _returnvalue_2 true (- 1.0 (* _returnvalue 0.8)) true))
  (:`Released`
    (`/Engine/EditorBlueprintResources/ActorMacros.Switch Has Authority`
      (:`Authority`
        _)
      (:`Remote`
        _))
    (`/HelicopterTestMaps/HeliFM.InputControls` _helifm _returnvalue_2 true 0.0 true)
    (set `self.IsUsingGamepad` false :!label _label_3)))

(event `Key|A`
  (params (Key :type "Key Structure" :default "AnyKey"))
  (bind _helifm (`self.HeliFM`))
  (bind _returnvalue (`KismetMathLibrary.Conv_BoolToInt` (`self.InvertControls`)))
  (bind _returnvalue_2 (- 3 _returnvalue))
  (:`Pressed`
    (`/Engine/EditorBlueprintResources/ActorMacros.Switch Has Authority`
      (:`Authority`
        _)
      (:`Remote`
        _))
    (`/HelicopterTestMaps/HeliFM.InputControls` _helifm _returnvalue_2 false (- 1.0 (* _returnvalue 0.8)) true))
  (:`Released`
    (`/Engine/EditorBlueprintResources/ActorMacros.Switch Has Authority`
      (:`Authority`
        _)
      (:`Remote`
        _))
    (`/HelicopterTestMaps/HeliFM.InputControls` _helifm _returnvalue_2 false 0.0 true)
    (goto _label_3)))

(event `Key|W`
  (params (Key :type "Key Structure" :default "AnyKey"))
  (:`Pressed`
    (`self.ServerSetW` true))
  (:`Released`
    (`self.ServerSetW` false)))

(event `ServerInputThrottle`
  (bind _keythrottle (`self.KeyThrottle`))
  (if (`/HelicopterTestMaps/HeliFM.IsHovering` (`self.HeliFM`))
    (if (not (`self.IsUsingGamepad`))
      (if (`self.IsKeyAdjusting`)
        (set `self.KeyThrottle` (`KismetMathLibrary.FClamp` (+ _keythrottle (* (`self.ThrottleDirection`) 0.03)) -1.0))
        (elif (not (== _keythrottle 0.0))
          (set `self.KeyThrottle` (`KismetMathLibrary.FClamp` (* (`KismetMathLibrary.SignOfFloat` _keythrottle) (- (`KismetMathLibrary.Abs` _keythrottle) 0.03)) -1.0))))
      (`/Engine/EditorBlueprintResources/ActorMacros.Switch Has Authority`
        (:`Authority`
          (`/HelicopterTestMaps/HeliFM.InputControls` (`self.HeliFM`) 0 false (`self.KeyThrottle`) false))))))

(event `ServerSetW`
  (params (Bool :type Boolean))
  (set `self.IsKeyAdjusting` Bool)
  (set `self.ThrottleDirection` 1)
  (set `self.IsUsingGamepad` false))

(event `InputAction|VehicleToggleEngine`
  (params (Key :type "Key Structure" :default "AnyKey"))
  (bind _helifm (`self.HeliFM`))
  (:`Pressed`
    (if (`self.bIsEngineActive`)
      (`/HelicopterTestMaps/HeliFM.StopEngine` _helifm)
      (elif (not (`/HelicopterTestMaps/HeliFM.StartingUp` _helifm))
        (`/HelicopterTestMaps/HeliFM.StartEngine` _helifm)
        (`KismetSystemLibrary.Delay` 3.0)
        (`SceneComponent.SetVisibility` (`self.ParticleSystem1`) true false)
        (`SceneComponent.SetVisibility` (`self.ParticleSystem_0`) true false)))))

(event `self.ReceiveTick`
  (params (DeltaSeconds :type "Float (single-precision)"))
  (bind (_returnvalue_x _returnvalue_y) (`KismetMathLibrary.BreakVector` (`self.GetVelocity`)))
  (bind (_returnvalue_roll _returnvalue_pitch) (`KismetMathLibrary.BreakRotator` (`self.K2_GetActorRotation`)))
  (bind _returnvalue (`SceneComponent.K2_GetComponentLocation` (`self.VehicleMesh`)))
  (bind _returnvalue_2 (+ _returnvalue (0.0 0.0 5.0)))
  (if (`self.bHasBeenDestroyed`)
    (if (not (`self.DestroyedWatcher`))
      (`self.SpawnWreck` (`self.GetVelocity`))
      (set `self.DestroyedWatcher` true)
      (bind _asrope_actor_2 (cast `/HelicopterTestMaps/Ropes/RopeActor_2` (`ChildActorComponent.ChildActor` (`self.Fastrope`)))
        (:`then`
          (bind _asrope_actor_2_2 (cast `/HelicopterTestMaps/Ropes/RopeActor_2` (`ChildActorComponent.ChildActor` (`self.Fastrope2`)))
            (:`then`
              (`/HelicopterTestMaps/Ropes/RopeActor_2.BreakRope` _asrope_actor_2)
              (`/HelicopterTestMaps/Ropes/RopeActor_2.BreakRope` _asrope_actor_2_2))
            (:`CastFailed`
              _)))
        (:`CastFailed`
          _))
      (`self.ServerSetDestroyed` true))
    (else
      (bind _asblack_hawk_screen_actor (cast `/HelicopterTestMaps/BlackhawkH_Backup/BlackHawkScreenActor` (`ChildActorComponent.ChildActor` (`self.BlackhawkScreen`))))
      (bind _outhit (`KismetSystemLibrary.LineTraceSingle` _returnvalue_2 (+ _returnvalue (0.0 0.0 -10000.0)) "TraceTypeQuery1"))
      (bind (_bblockinghit _binitialoverlap _time _location) (`GameplayStatics.BreakHitResult` _outhit))
      (bind _z (.z (- _location _returnvalue_2)))
      (set `self.Altitude` _z)
      (set `self.DustTransform` (`KismetMathLibrary.Conv_VectorToTransform` _location))
      (`/HelicopterTestMaps/BlackhawkH_Backup/BlackHawkScreenActor.UpdatePitchWidget` _asblack_hawk_screen_actor (`KismetMathLibrary.FClamp` _returnvalue_pitch -50.0 50.0) _returnvalue_roll (* (`KismetMathLibrary.FTrunc` _z) -1) (`/HelicopterTestMaps/HeliFM.Throttle` (`self.HeliFM`)) (`KismetMathLibrary.VSize` (`KismetMathLibrary.MakeVector` _returnvalue_x _returnvalue_y)) (`self.InvertControls`) 0 (`self.DeployedRopes`))
      (if (not (`self.IsUsingGamepad`))
        (`self.ServerInputThrottle`)))))

(event `ServerHandBrake`
  (if (`self.canBreak`)
    (set `self.canBreak` false)
    (bind _asrope_actor_2 (cast `/HelicopterTestMaps/Ropes/RopeActor_2` (`ChildActorComponent.ChildActor` (`self.Fastrope`))))
    (bind _asrope_actor_2_2 (cast `/HelicopterTestMaps/Ropes/RopeActor_2` (`ChildActorComponent.ChildActor` (`self.Fastrope2`))))
    (if (`self.DeployedRopes`)
      (`/HelicopterTestMaps/Ropes/RopeActor_2.BreakRope` _asrope_actor_2)
      (`/HelicopterTestMaps/Ropes/RopeActor_2.BreakRope` _asrope_actor_2_2)
      (set `self.DeployedRopes` false)
      (`KismetSystemLibrary.Delay` 2.0)
      (set `self.canBreak` true)
      (else
        (`/HelicopterTestMaps/Ropes/RopeActor_2.DeployRope` _asrope_actor_2)
        (`/HelicopterTestMaps/Ropes/RopeActor_2.DeployRope` _asrope_actor_2_2)
        (set `self.DeployedRopes` true)
        (`KismetSystemLibrary.Delay` 2.0)
        (set `self.canBreak` true)))))

(event `InputAction|VehicleHandbrake`
  (params (Key :type "Key Structure" :default "AnyKey"))
  (:`Pressed`
    (`self.ServerHandBrake`)))

(event `self.ReceiveBeginPlay`
  (`ActorComponent.Activate` (`self.Camera`) false)
  (`ActorComponent.Deactivate` (`self.ExternalCamera`)))

(event `InputAction|ToggleView`
  (params (Key :type "Key Structure" :default "AnyKey"))
  (bind _externalcamera (`self.ExternalCamera`))
  (bind _camera (`self.Camera`))
  (:`Pressed`
    (if (`SQBlueprintLibrary.IsShippingBuild`)
      _
      (elif (`ActorComponent.IsActive` (`self.Camera`))
        (`ActorComponent.Deactivate` _camera)
        (`ActorComponent.Activate` _externalcamera false)
        (else
          (`ActorComponent.Activate` _camera false)
          (`ActorComponent.Deactivate` _externalcamera))))))

(event `self.LeftVehicle`
  (params (Soldier :type "SQSoldier Object Reference") (PreviousSeat :type "SQVehicleSeatComponent Object Reference"))
  (bind _assqplayer_controller (cast `SQPlayerController` (`self.GetController` Soldier)))
  (`/Engine/EditorBlueprintResources/ActorMacros.Switch Has Authority`
    (:`Authority`
      (`self.PickRopeMount` _assqplayer_controller))))

(event `SpawnWreck`
  (params (Vel :type "Vector Structure"))
  (bind _returnvalue (`|SpawnActorFromClass` "/HelicopterTestMaps/BlackhawkH_2/Blackhawk_Wreckage3.Blackhawk_Wreckage3_C" (`self.GetTransform`) "AlwaysSpawn" "OverrideRootScale" null "Team_Neutral"))
  (`PrimitiveComponent.AddImpulse` (`SQVehicle.VehicleMesh` _returnvalue) Vel "None" true)
  (`KismetSystemLibrary.Delay` 300.0)
  (`/Engine/EditorBlueprintResources/StandardMacros.IsValid` _returnvalue
    (:`Is Valid`
      (`self.K2_DestroyActor` _returnvalue))))

(event `PickRopeMount`
  (params (Controller :type "SQPlayerController Object Reference"))
  (bind _asrope_actor_2 (cast `/HelicopterTestMaps/Ropes/RopeActor_2` (`ChildActorComponent.ChildActor` (`self.Fastrope`))))
  (bind _seattaken (`/HelicopterTestMaps/Ropes/RopeActor_2.CanMount` _asrope_actor_2))
  (if _seattaken
    (bind _asrope_actor_2_2 (cast `/HelicopterTestMaps/Ropes/RopeActor_2` (`ChildActorComponent.ChildActor` (`self.Fastrope2`))))
    (bind _seattaken_2 (`/HelicopterTestMaps/Ropes/RopeActor_2.CanMount` _asrope_actor_2_2))
    (if _seattaken_2
      (if (`self.DeployedRopes`)
        _)
      (else
        (`/HelicopterTestMaps/Ropes/RopeActor_2.ServerOnUsed` _asrope_actor_2_2 Controller)
        (set `/HelicopterTestMaps/Ropes/RopeActor_2.ClimbLength` 1.0 _asrope_actor_2_2)))
    (else
      (`/HelicopterTestMaps/Ropes/RopeActor_2.ServerOnUsed` _asrope_actor_2 Controller)
      (set `/HelicopterTestMaps/Ropes/RopeActor_2.ClimbLength` 1.0 _asrope_actor_2))))

(event `InputAxisKey|MouseY`
  (params (AxisValue :type "Float (single-precision)"))
  (bind _pitchlimit (`self.PitchLimit`))
  (bind _returnvalue (* (`self.PitchLimit`) -1.0))
  (bind (_relativerotation_roll _relativerotation_pitch) (`KismetMathLibrary.BreakRotator` (`SceneComponent.RelativeRotation` (`self.Camera`))))
  (bind _returnvalue_2 (select `bool` (>= _relativerotation_pitch 180.0) :`false` _relativerotation_pitch :`true` (- _relativerotation_pitch 360.0)))
  ;[1 1 1] Driver Head Rotation
  (if (`self.Free Looking`)
    (`SceneComponent.K2_AddRelativeRotation` (`self.Camera`) (`KismetMathLibrary.MakeRotator` 0.0 (`KismetMathLibrary.FClamp` AxisValue (`KismetMathLibrary.FClamp` (- _returnvalue _returnvalue_2) _returnvalue 0.0) (`KismetMathLibrary.FClamp` (- _pitchlimit _returnvalue_2) 0.0 _pitchlimit))) false false)))

(event `InputAxis|Turn`
  (params (AxisValue :type "Float (single-precision)"))
  (bind _camera (`self.Camera`))
  (bind _yawlimit (`self.YawLimit`))
  (bind _returnvalue (* _yawlimit -1.0))
  (bind (_relativerotation_roll _relativerotation_pitch _relativerotation_yaw) (`KismetMathLibrary.BreakRotator` (`SceneComponent.RelativeRotation` (`self.Camera`))))
  (bind _returnvalue_2 (select `bool` (>= _relativerotation_yaw 180.0) :`false` _relativerotation_yaw :`true` (- _relativerotation_yaw 360.0)))
  ;[1 1 1] Driver Head Rotation
  (if (`self.Free Looking`)
    (`SceneComponent.K2_AddRelativeRotation` _camera (`KismetMathLibrary.MakeRotator` 0.0 0.0 (`KismetMathLibrary.FClamp` AxisValue (`KismetMathLibrary.FClamp` (- _returnvalue _returnvalue_2) _returnvalue 0.0) (`KismetMathLibrary.FClamp` (- _yawlimit _returnvalue_2) 0.0 _yawlimit))) false false)
    (else
      (`SceneComponent.K2_SetRelativeRotation` :`self` _camera))))

(fn `CanUnmount`
  (returns (CanUnmount :type Boolean))
  (if (`self.DeployedRopes`)
    (bind _asrope_actor_2 (cast `/HelicopterTestMaps/Ropes/RopeActor_2` (`ChildActorComponent.ChildActor` (`self.Fastrope`))))
    (bind _seattaken (`/HelicopterTestMaps/Ropes/RopeActor_2.CanMount` _asrope_actor_2))
    (if _seattaken
      (bind _asrope_actor_2_2 (cast `/HelicopterTestMaps/Ropes/RopeActor_2` (`ChildActorComponent.ChildActor` (`self.Fastrope2`))))
      (bind _seattaken_2 (`/HelicopterTestMaps/Ropes/RopeActor_2.CanMount` _asrope_actor_2_2))
      (if _seattaken_2
        (return false)
        (else
          _))))
  (return true))

(fn `IncEngine`
  (params (Int :type "Float (double-precision)") (Min :type "Float (double-precision)") (WarmupBypass :type Boolean))
  (bind _enginepower (`self.EnginePower`))
  (if (> 0.0 Int)
    _
    (else
      _))
  (if (`self.warmedUp`)
    (set `self.EnginePower` (`KismetMathLibrary.FClamp` (+ (`self.EnginePower`) Int) Min 8.0) :!label _label)
    (`self.ServerSetFloatParam` _enginepower)
    (`AudioComponent.SetFloatParameter` (`self.EngineSpeedAC`) "EngineSpeed" _enginepower)
    (`AudioComponent.SetFloatParameter` (`self.EngineRPMAC`) "EngineSpeed" _enginepower)
    (elif WarmupBypass
      (goto _label))))

(fn `SpawnWreckage`
  (params (Velocity :type "Vector Structure"))
  (bind _returnvalue (`|SpawnActorFromClass` "/HelicopterTestMaps/BlackhawkH_Backup/wreckage/BlackhawkWreckage.BlackhawkWreckage_C" (`self.GetTransform`) "AlwaysSpawn" "OverrideRootScale"))
  (`self.K2_DestroyActor`)
  (`PrimitiveComponent.AddImpulse` (`/HelicopterTestMaps/BlackhawkH_Backup/wreckage/BlackhawkWreckage.SkeletalMesh` _returnvalue) Velocity "None" true))

(fn `UserConstructionScript`)