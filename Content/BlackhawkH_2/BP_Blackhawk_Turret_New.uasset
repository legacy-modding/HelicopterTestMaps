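; Player-controlled Blackhawk helicopter gun turret for Squad, handling aiming, firing, focus zoom and freelook.
; Turn and LookUp feed clamped controller input within yaw and pitch limits, with elevation also speed-capped and gated on weapon input and a living soldier.
; Tick drives freelook by ignoring look input and rotating the camera within its own limits, then resets camera and controller state when local control ends.
; Overrides supply attach and camera components, and construction wires the static turret movement component.
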(event `InputAction|FreeLook`
  (params (Key :type "Key Structure" :default "AnyKey"))
  ;[0 0 0] Freelook
  (:`Pressed`
    (set `self.bIsFreelooking` true))
  (:`Released`
    (set `self.bIsFreelooking` false)))

(event `SetControllerReference`
  ;[0 0 0] Freelook
  (`/Engine/EditorBlueprintResources/StandardMacros.IsValid` (`self.ControllerRef`)
    (:`Is Not Valid`
      (bind _assqplayer_controller (cast `SQPlayerController` (`self.GetOwner`)))
      (set `self.ControllerRef` _assqplayer_controller))))

(event `self.ReceiveTick`
  (params (DeltaSeconds :type "Float (single-precision)"))
  ;[0 0 0] Freelook
  (if (`self.IsLocallyControlled`)
    (`self.SetControllerReference`)
    (`|ExecutionSequence`
      (:`then_0`
        (if (`self.bIsFreelooking`)
          (`self.TurretFreelook`)
          (goto _label :!via `Reset`)
          (else
            (`/Engine/EditorBlueprintResources/StandardMacros.DoOnce` false :!label _label
              (:`Completed`
                (`self.ResetFreelook`))))))
      (:`then_1`
        (`self.ResetDoOnce`)))
    (else
      (`/Engine/EditorBlueprintResources/StandardMacros.DoOnce` false :!label _label_2
        (:`Completed`
          (`self.LeaveEmplacement`))))))

(event `ResetDoOnce`
  ;[0 0 0] Freelook
  (goto _label_2 :!via `Reset`))

(event `LeaveEmplacement`
  (bind _controllerref (`self.ControllerRef`))
  ;[0 0 0] Freelook
  (`self.ResetFreelook`)
  (set `self.bIsFreelooking` false)
  (`/Engine/EditorBlueprintResources/StandardMacros.IsValid` _controllerref
    (:`Is Valid`
      (bind _assqsoldier_new (cast `SQSoldierNew` (`Controller.K2_GetPawn` _controllerref)))
      (set `SQSoldierNew.bIsUsingFreeLook` false _assqsoldier_new)
      (set `self.ControllerRef` null))))

(event `ResetFreelook`
  (bind _controllerref (`self.ControllerRef`))
  ;[0 0 0] Freelook
  (`SceneComponent.K2_SetRelativeRotation` :`self` (`self.Camera`))
  (`/Engine/EditorBlueprintResources/StandardMacros.IsValid` _controllerref
    (:`Is Valid`
      (`Controller.ResetIgnoreLookInput` _controllerref))))

(event `TurretFreelook`
  (bind _controllerref (`self.ControllerRef`))
  (bind _camera (`self.Camera`))
  (bind (_x _y) (`KismetMathLibrary.BreakVector2D` (`self.FreelookLimitYaw`)))
  (bind (_x_2 _y_2) (`KismetMathLibrary.BreakVector2D` (`self.FreelookLimitPitch`)))
  ;[0 0 0] Freelook
  (`/Engine/EditorBlueprintResources/StandardMacros.IsValid` _controllerref
    (:`Is Valid`
      (`Controller.SetIgnoreLookInput` _controllerref true)
      (`SceneComponent.K2_SetRelativeRotation` _camera (`KismetMathLibrary.MakeRotator` 0.0 (`KismetMathLibrary.FClamp` (+ (.pitch (`SceneComponent.RelativeRotation` _camera)) (* (* (`SQGameUserSettings.FreelookSensitivity` (`SQBlueprintLibrary.GetSquadGameUserSettings`)) (`self.GetInputAxisValue`)) -1.0)) _x_2 _y_2) (`KismetMathLibrary.FClamp` (+ (.yaw (`SceneComponent.RelativeRotation` _camera)) (* (`SQGameUserSettings.FreelookSensitivity` (`SQBlueprintLibrary.GetSquadGameUserSettings`)) (`self.GetInputAxisValue`))) _x _y)) false false))))

(event `self.ReceiveUnpossessed`
  (params (OldController :type "Controller Object Reference"))
  (`self.ResetFreelook`))

(event `InputAction|Focus`
  (params (Key :type "Key Structure" :default "AnyKey"))
  (bind _fov (`SQGameUserSettings.FOV` (`SQBlueprintLibrary.GetSquadGameUserSettings`)))
  ;[1 1 1] Focus FOV shift
  (:`Pressed`
    (`CameraComponent.SetFieldOfView` (`self.Camera`) (* 0.666 _fov)))
  (:`Released`
    (`CameraComponent.SetFieldOfView` (`self.Camera`) _fov)))

(event `InputAxis|Turn`
  (params (AxisValue :type "Float (single-precision)"))
  (bind (_returnvalue_roll _returnvalue_pitch _returnvalue_yaw) (`KismetMathLibrary.BreakRotator` (`self.GetControlRotation`)))
  (bind _yawlimit (`self.YawLimit`))
  (bind _returnvalue (* _yawlimit -1.0))
  (bind _returnvalue_2 (select `bool` (>= _returnvalue_yaw 180.0) :`false` _returnvalue_yaw :`true` (- _returnvalue_yaw 360.0)))
  (`self.AddControllerYawInput` (`KismetMathLibrary.FClamp` AxisValue (`KismetMathLibrary.FClamp` (- _returnvalue _returnvalue_2) _returnvalue 0.0) (`KismetMathLibrary.FClamp` (- _yawlimit _returnvalue_2) 0.0 _yawlimit))))

(event `InputAxis|LookUp`
  (params (AxisValue :type "Float (single-precision)"))
  (bind (_returnvalue_roll _returnvalue_pitch) (`KismetMathLibrary.BreakRotator` (`self.GetControlRotation`)))
  (bind _pitchlimit (`self.PitchLimit`))
  (bind _maxelevationspeed (`self.MaxElevationSpeed`))
  (bind _minpitchlimit (`self.MinPitchLimit`))
  (bind _returnvalue (* (select `bool` (>= _returnvalue_pitch 180.0) :`false` _returnvalue_pitch :`true` (- _returnvalue_pitch 360.0)) -1.0))
  (if (not (`self.bIsFreelooking`))
    (bind _binputenabled (`self.IsCurrentWeaponInputEnabled`))
    (if _binputenabled
      (`self.AddControllerPitchInput` (`KismetMathLibrary.FClamp` (`KismetMathLibrary.FClamp` (* AxisValue (`self.ElevationSpeedMultiplier`)) (* _maxelevationspeed -1.0) _maxelevationspeed) (`KismetMathLibrary.FClamp` (- _minpitchlimit _returnvalue) _minpitchlimit 0.0) (`KismetMathLibrary.FClamp` (- _pitchlimit _returnvalue) 0.0 _pitchlimit))))))

(event `InputAction|Fire`
  (params (Key :type "Key Structure" :default "AnyKey"))
  (bind _currentweapon (`SQPawnInventoryComponent.CurrentWeapon` (`self.GetVehicleInventory`)))
  (:`Pressed`
    (`SQEquipableItem.BeginUse` _currentweapon))
  (:`Released`
    (`SQEquipableItem.EndUse` _currentweapon)))

(fn `Get1PAttachComponent`
  (returns (ReturnValue :type "SceneComponent Object Reference"))
  (return (`self.GunAttachPoint`)))

(fn `Get3PAttachComponent`
  (returns (ReturnValue :type "SceneComponent Object Reference"))
  (return (`self.GunAttachPoint`)))

(fn `GetADSCameraLocationComponent`
  (returns (ReturnValue :type "SceneComponent Object Reference"))
  (return (`self.ADSCameraPosition`)))

(fn `GetDefaultCameraLocationComponent`
  (returns (ReturnValue :type "SceneComponent Object Reference"))
  (return (`self.DefaultCameraPosition`)))

(fn `GetMasterPoseComponent`
  (returns (ReturnValue :type "SkinnedMeshComponent Object Reference"))
  (return null))

(fn `GetSoldierAttachComponent`
  (returns (ReturnValue :type "SceneComponent Object Reference"))
  (return (`SQVehicle.VehicleMesh` (`self.GetVehicle`))))

(fn `GetWeaponAttachComponent`
  (returns (ReturnValue :type "SceneComponent Object Reference"))
  (return (`self.GunAttachPoint`)))

(fn `IsCurrentWeaponInputEnabled`
  (returns (bInputEnabled :type Boolean))
  (bind _sqvehicleinventory (`self.SQVehicleInventory`)
    (:`then`
      (bind _assqvehicle_weapon (cast `SQVehicleWeapon` (`SQPawnInventoryComponent.CurrentWeapon` _sqvehicleinventory))
        (:`then`
          (if (`SQVehicleWeapon.bInputEnabled` _assqvehicle_weapon)
            (bind _returnvalue (`self.IsSoldierAlive`))
            (if _returnvalue
              (return true)
              (else
                (return false)))
            (else
              (return false))))
        (:`CastFailed`
          (return false))))
    (:`else`
      (return false))))

(fn `IsSoldierAlive`
  (returns (ReturnValue :type Boolean))
  (bind _currentweapon (`SQPawnInventoryComponent.CurrentWeapon` (`self.SQVehicleInventory`))
    (:`then`
      (bind _assqvehicle_weapon (cast `SQVehicleWeapon` _currentweapon)
        (:`then`
          (bind _returnvalue (`SQVehicleWeapon.GetSoldier` _assqvehicle_weapon))
          (`/Engine/EditorBlueprintResources/StandardMacros.IsValid` _returnvalue
            (:`Is Valid`
              (return (`SQSoldier.IsAlive` _returnvalue)))
            (:`Is Not Valid`
              (return false))))
        (:`CastFailed`
          (return false))))
    (:`else`
      (return false))))

(fn `UserConstructionScript`
  (set `SQStaticTurretMovementComponent.YawComponent` (`self.Turret_SkeletalMesh`) (`self.SQStaticTurretMovement`))
  (set `SQStaticTurretMovementComponent.PitchComponent` (`self.GunAttachPoint`) (`self.SQStaticTurretMovement`)))