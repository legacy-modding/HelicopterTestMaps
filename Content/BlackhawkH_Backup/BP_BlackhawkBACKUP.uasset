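; Player-flown Blackhawk helicopter vehicle (backup copy) with physics-driven flight, engine warmup and a cockpit instrument screen.
; Inputs feed Server-named events for throttle, pitch and yaw; Tick turns EnginePower into upward impulses and banking, though descend only sets a flag.
; IncEngine drives engine audio behind a warmup gate, stepped by a ForLoopDelay macro on startup, while RotorSpin animates blades.
; Also handles free-look, a non-shipping external camera and impact damage.
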(event `ServerIncEngine`
  (params (Int :type "Float (double-precision)") (Min :type "Float (double-precision)") (Bypass :type Boolean))
  (`self.IncEngine` Int Min Bypass))

(event `ServerSetHover`
  (params (NewParam :type Integer))
  (set `self.engineHover` NewParam))

(event `ServerSetWarmup`
  (params (NewParam :type Boolean))
  (set `self.warmedUp` NewParam))

(event `ServerSetControls`
  (params (Control :type Integer) (Bool :type Boolean))
  (switch `int` Control
    (:`Default`
      (set `self.EngineForward` Bool :!label _label))
    (:`0`
      (set `self.isDescending` Bool))
    (:`1`
      (set `self.turnRight` Bool))
    (:`2`
      (set `self.turnLeft` Bool))
    (:`3`
      (goto _label))))

(event `Key|S`
  (params (Key :type "Key Structure" :default "AnyKey"))
  (:`Pressed`
    (`self.ServerSetControls` 0 true))
  (:`Released`
    (`self.ServerSetControls` 0)))

(event `ServerSetPitch`
  (params (Pitch :type "Float (double-precision)"))
  (bind _elevation_maxspeed (`self.Elevation MaxSpeed`))
  (bind _vehiclemesh (`self.VehicleMesh`))
  (`PrimitiveComponent.AddAngularImpulse` _vehiclemesh (* (`SceneComponent.GetRightVector` _vehiclemesh) (`KismetMathLibrary.FClamp` (* Pitch (`self.Elevation Speed`)) (* _elevation_maxspeed -1.0) _elevation_maxspeed)) "None" true))

(event `Key|D`
  (params (Key :type "Key Structure" :default "AnyKey"))
  (:`Pressed`
    (`self.ServerSetControls` 1 true))
  (:`Released`
    (`self.ServerSetControls` 1)))

(event `Key|A`
  (params (Key :type "Key Structure" :default "AnyKey"))
  (:`Pressed`
    (`self.ServerSetControls` 2 true))
  (:`Released`
    (`self.ServerSetControls` 2)))

(event `ServerSetYaw`
  (params (Yaw :type "Float (double-precision)"))
  (bind _yaw_maxspeed (`self.Yaw MaxSpeed`))
  (`PrimitiveComponent.SetPhysicsAngularVelocity` (`self.VehicleMesh`) (`KismetMathLibrary.MakeVector` 0.0 0.0 (`KismetMathLibrary.FClamp` (* Yaw (`self.Yaw Speed`)) (* _yaw_maxspeed -1.0) _yaw_maxspeed)) true "None"))

(event `Key|W`
  (params (Key :type "Key Structure" :default "AnyKey"))
  (:`Pressed`
    (`self.ServerSetControls` 3 true))
  (:`Released`
    (`self.ServerSetControls` 3)))

(event `InputAction|VehicleToggleEngine`
  (params (Key :type "Key Structure" :default "AnyKey"))
  (:`Pressed`
    (if (not (`self.bIsEngineActive`))
      (`KismetSystemLibrary.Delay` 1.0)
      (bind _index (`self.ForLoopDelay` 0 5 3.0)
        (:`LoopBody`
          (`self.ServerIncEngine` 1.0 0.0 true))
        (:`Completed`
          (`KismetSystemLibrary.Delay` 5.0)
          (`self.ServerSetWarmup` true)))
      (`self.ServerSetHover` _index))))

(event `self.ReceiveTick`
  (params (DeltaSeconds :type "Float (single-precision)"))
  (bind (_returnvalue_roll _returnvalue_pitch) (`KismetMathLibrary.BreakRotator` (`self.K2_GetActorRotation`)))
  (bind _vehiclemesh (`self.VehicleMesh`))
  (bind _vehiclemesh_2 (`self.VehicleMesh`))
  (bind _returnvalue (`SceneComponent.K2_GetComponentLocation` (`self.VehicleMesh`)))
  (bind _returnvalue_2 (`KismetMathLibrary.Conv_IntToDouble` (`self.engineHover`)))
  (bind _returnvalue_3 (* (`SceneComponent.GetForwardVector` _vehiclemesh_2) 0.01))
  (bind _returnvalue_4 (+ _returnvalue (0.0 0.0 5.0)))
  (bind _asblack_hawk_screen_actor (cast `/HelicopterTestMaps/BlackhawkH_Backup/BlackHawkScreenActor` (`ChildActorComponent.ChildActor` (`self.BlackhawkScreen`))))
  (bind _outhit (`KismetSystemLibrary.LineTraceSingle` :`Start` _returnvalue_4 :`End` (+ _returnvalue (0.0 0.0 -10000.0)) :`TraceChannel` "TraceTypeQuery1" :`DrawDebugType` "ForOneFrame"))
  (`/HelicopterTestMaps/BlackhawkH_Backup/BlackHawkScreenActor.UpdatePitchWidget` _asblack_hawk_screen_actor (`KismetMathLibrary.FClamp` _returnvalue_pitch -50.0 50.0) _returnvalue_roll (`KismetMathLibrary.FTrunc` (.z (- (`.Location` (`GameplayStatics.BreakHitResult` _outhit)) _returnvalue_4))) (`self.EnginePower`) (`KismetMathLibrary.VSize` (`self.GetVelocity`)) false 0 false)
  (if (`self.bIsEngineActive`)
    _
    (elif (`self.IsEngineActive`)
      (`KismetSystemLibrary.Delay` 1.0)
      (set `self.warmedUp` true)
      (set `self.engineHover` 5)))
  (`self.RotorSpin` (`self.EnginePower`))
  (if (`self.bIsEngineActive`)
    (if (`self.EngineForward`)
      (`self.IncEngine` 0.02 _returnvalue_2)
      (`PrimitiveComponent.AddImpulse` (`self.VehicleMesh`) (* (* (* (`KismetMathLibrary.GetUpVector` (`SceneComponent.K2_GetComponentRotation` _vehiclemesh_2)) (* (`self.EnginePower`) 2.0)) DeltaSeconds) 75) "None" true)
      (if (`self.turnLeft`)
        (`PrimitiveComponent.AddAngularImpulse` _vehiclemesh _returnvalue_3 "None" true)
        (elif (`self.turnRight`)
          (`PrimitiveComponent.AddAngularImpulse` _vehiclemesh (* _returnvalue_3 -1) "None" true)))
      (else
        (if (`self.isDescending`)
          _
          (else
            _))
        (`self.IncEngine` -0.01 _returnvalue_2)))
    (else
      (`self.IncEngine` -0.02))))

(event `ServerUpdatePosition`
  (params (UpdatedTransform :type "Transform Structure")))

(event `OnTakeAnyDamage_Event_1` :!signature `self.OnTakeAnyDamage`
  (params (DamagedActor :type "Actor Object Reference") (Damage :type "Float (double-precision)") (DamageType :type "DamageType Object Reference") (InstigatedBy :type "Controller Object Reference") (DamageCauser :type "Actor Object Reference"))
  ;[1 1 1] Burning Effects Setup
  (bind _assqdamage_type (cast `SQDamageType` DamageType)))

(event `self.ReceiveBeginPlay`
  (`ActorComponent.Activate` (`self.Camera`) false)
  (`ActorComponent.Deactivate` (`self.ExternalCamera`)))

(event `InputAxis|LookUp`
  (params (AxisValue :type "Float (single-precision)"))
  (bind _elevation_maxspeed (`self.Elevation MaxSpeed`))
  (if (`ActorComponent.IsActive` (`self.ExternalCamera`))
    _
    (elif (not (`self.FreeLooking`))
      (`self.ServerSetPitch` (`KismetMathLibrary.FClamp` (* AxisValue (`self.Elevation Speed`)) (* _elevation_maxspeed -1.0) _elevation_maxspeed)))))

(event `self.VehicleMesh.OnComponentHit`
  (params (HitComponent :type "PrimitiveComponent Object Reference") (OtherActor :type "Actor Object Reference") (OtherComp :type "PrimitiveComponent Object Reference") (NormalImpulse :type "Vector Structure") (Hit :type "HitResult Structure (by ref)"))
  (bind _returnvalue (`KismetMathLibrary.VSize` NormalImpulse))
  (if (> _returnvalue (`self.minImpactSpeed`))
    (`GameplayStatics.ApplyDamage` self (* 100 (/ _returnvalue (`self.minImpactSpeed`))) null null "/Script/Squad.SQBurningDamage")))

(event `InputAction|ToggleView`
  (params (Key :type "Key Structure" :default "AnyKey"))
  (bind _camera (`self.Camera`))
  (bind _externalcamera (`self.ExternalCamera`))
  (:`Pressed`
    (if (`SQBlueprintLibrary.IsShippingBuild`)
      _
      (elif (`ActorComponent.IsActive` (`self.Camera`))
        (`ActorComponent.Deactivate` _camera)
        (`ActorComponent.Activate` _externalcamera false)
        (else
          (`ActorComponent.Activate` _camera false)
          (`ActorComponent.Deactivate` _externalcamera))))))

(event `Key|MouseScrollUp`
  (params (Key :type "Key Structure" :default "AnyKey"))
  (bind _springarm (`self.SpringArm`))
  (:`Pressed`
    (if (`ActorComponent.IsActive` (`self.ExternalCamera`))
      (set `SpringArmComponent.TargetArmLength` (`KismetMathLibrary.FMax` (- (`SpringArmComponent.TargetArmLength` _springarm) 25.0)) _springarm))))

(event `InputAxisKey|MouseX`
  (params (AxisValue :type "Float (single-precision)"))
  (if (`ActorComponent.IsActive` (`self.ExternalCamera`))
    _
    (elif (not (`self.FreeLooking`))
      (`self.ServerSetYaw` AxisValue))))

(event `Key|MouseScrollDown`
  (params (Key :type "Key Structure" :default "AnyKey"))
  (bind _springarm (`self.SpringArm`))
  (:`Pressed`
    (if (`ActorComponent.IsActive` (`self.ExternalCamera`))
      (set `SpringArmComponent.TargetArmLength` (`KismetMathLibrary.FClamp` (+ (`SpringArmComponent.TargetArmLength` _springarm) 25.0) 0.0 800.0) _springarm))))

(event `Key|LeftAlt`
  (params (Key :type "Key Structure" :default "AnyKey"))
  ;[1 1 1] Driver Head Rotation
  (:`Pressed`
    (set `self.FreeLooking` true))
  (:`Released`
    (set `self.FreeLooking` false)))

(event `InputAxis|Turn`
  (params (AxisValue :type "Float (single-precision)"))
  (bind _camera (`self.Camera`))
  (bind _yawlimit (`self.YawLimit`))
  (bind _returnvalue (* _yawlimit -1.0))
  (bind (_relativerotation_roll _relativerotation_pitch _relativerotation_yaw) (`KismetMathLibrary.BreakRotator` (`SceneComponent.RelativeRotation` (`self.Camera`))))
  (bind _returnvalue_2 (select `bool` (>= _relativerotation_yaw 180.0) :`false` _relativerotation_yaw :`true` (- _relativerotation_yaw 360.0)))
  ;[1 1 1] Driver Head Rotation
  (if (`self.FreeLooking`)
    (`SceneComponent.K2_AddRelativeRotation` _camera (`KismetMathLibrary.MakeRotator` 0.0 0.0 (`KismetMathLibrary.FClamp` AxisValue (`KismetMathLibrary.FClamp` (- _returnvalue _returnvalue_2) _returnvalue 0.0) (`KismetMathLibrary.FClamp` (- _yawlimit _returnvalue_2) 0.0 _yawlimit))) false false)
    (else
      (`SceneComponent.K2_SetRelativeRotation` :`self` _camera))))

(fn `IncEngine`
  (params (Int :type "Float (double-precision)") (Min :type "Float (double-precision)") (WarmupBypass :type Boolean))
  (bind _enginepower (`self.EnginePower`))
  (if (> 0.0 Int)
    _
    (else
      _))
  (if (`self.warmedUp`)
    (set `self.EnginePower` (`KismetMathLibrary.FClamp` (+ (`self.EnginePower`) Int) Min 8.0) :!label _label)
    (`AudioComponent.SetFloatParameter` (`self.EngineRPMAC`) "EngineSpeed" _enginepower)
    (`AudioComponent.SetFloatParameter` (`self.EngineSpeedAC`) "EngineSpeed" _enginepower)
    (elif WarmupBypass
      (goto _label))))

(fn `RotorSpin`
  (params (Speed :type "Float (double-precision)"))
  (bind _returnvalue (* Speed 5.0))
  (`SceneComponent.K2_AddLocalRotation` (`self.RotorBlade1`) (`KismetMathLibrary.MakeRotator` 0.0 0.0 _returnvalue) false false)
  (`SceneComponent.K2_AddLocalRotation` (`self.TailRotor`) (`KismetMathLibrary.MakeRotator` 0.0 _returnvalue) false false))

(fn `UserConstructionScript`)