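; Player-controlled Blackhawk turret pawn that aims and fires the current vehicle weapon.
; Look and turn input is clamped to pitch and yaw limits, and applies only while the weapon accepts input and its soldier is alive.
; Construction binds static turret movement to the root for yaw and the gun attach point for pitch.
; Focus narrows camera FOV, and non-shipping builds can toggle an orbiting, zoomable third-person debug camera.
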(event `InputAction|ToggleView`
  (params (Key :type "Key Structure" :default "AnyKey"))
  (bind _camera (`self.Camera`))
  (bind _externalcamera (`self.ExternalCamera`))
  ;[1 1 1] Third Person Debug Camera
  (:`Pressed`
    (if (`SQBlueprintLibrary.IsShippingBuild`)
      _
      (elif (`ActorComponent.IsActive` (`self.Camera`))
        (`ActorComponent.Deactivate` _camera)
        (`ActorComponent.Activate` _externalcamera false)
        (else
          (`ActorComponent.Activate` _camera false)
          (`ActorComponent.Deactivate` _externalcamera))))))

(event `Key|MouseScrollUp`
  (params (Key :type "Key Structure" :default "AnyKey"))
  (bind _spring_arm (`self.Spring Arm`))
  ;[1 1 1] Third Person Debug Camera
  (:`Pressed`
    (if (`ActorComponent.IsActive` (`self.ExternalCamera`))
      (set `SpringArmComponent.TargetArmLength` (`KismetMathLibrary.FMax` (- (`SpringArmComponent.TargetArmLength` _spring_arm) 25.0)) _spring_arm))))

(event `Key|MouseScrollDown`
  (params (Key :type "Key Structure" :default "AnyKey"))
  (bind _spring_arm (`self.Spring Arm`))
  ;[1 1 1] Third Person Debug Camera
  (:`Pressed`
    (if (`ActorComponent.IsActive` (`self.ExternalCamera`))
      (set `SpringArmComponent.TargetArmLength` (+ (`SpringArmComponent.TargetArmLength` _spring_arm) 25.0) _spring_arm))))

(event `InputAxisKey|MouseX`
  (params (AxisValue :type "Float (single-precision)"))
  ;[1 1 1] Third Person Debug Camera
  (if (`ActorComponent.IsActive` (`self.ExternalCamera`))
    (`SceneComponent.K2_AddLocalRotation` (`self.Spring Arm`) (`KismetMathLibrary.MakeRotator` 0.0 0.0 AxisValue) false false)))

(event `InputAxisKey|MouseY`
  (params (AxisValue :type "Float (single-precision)"))
  ;[1 1 1] Third Person Debug Camera
  (if (`ActorComponent.IsActive` (`self.ExternalCamera`))
    (`SceneComponent.K2_AddLocalRotation` (`self.Spring Arm`) (`KismetMathLibrary.MakeRotator` 0.0 AxisValue) false false)))

(event `InputAction|Focus`
  (params (Key :type "Key Structure" :default "AnyKey"))
  (bind _fov (`SQGameUserSettings.FOV` (`SQBlueprintLibrary.GetSquadGameUserSettings`)))
  ;[1 1 1] Focus FOV shift
  (:`Pressed`
    (`CameraComponent.SetFieldOfView` (`self.Camera`) (* 0.666 _fov)))
  (:`Released`
    (`CameraComponent.SetFieldOfView` (`self.Camera`) _fov)))

(event `InputAxis|LookUp`
  (params (AxisValue :type "Float (single-precision)"))
  (bind (_returnvalue_roll _returnvalue_pitch) (`KismetMathLibrary.BreakRotator` (`self.GetControlRotation`)))
  (bind _pitchlimit (`self.PitchLimit`))
  (bind _returnvalue (* (`self.PitchUpLimit`) -1.0))
  (bind _returnvalue_2 (* (select `bool` (>= _returnvalue_pitch 180.0) :`false` _returnvalue_pitch :`true` (- _returnvalue_pitch 360.0)) -1.0))
  (bind _binputenabled (`self.IsCurrentWeaponInputEnabled`))
  (if _binputenabled
    (`self.AddControllerPitchInput` (`KismetMathLibrary.FClamp` AxisValue (`KismetMathLibrary.FClamp` (- _returnvalue _returnvalue_2) _returnvalue 0.0) (`KismetMathLibrary.FClamp` (- _pitchlimit _returnvalue_2) 0.0 _pitchlimit)))))

(event `InputAxis|Turn`
  (params (AxisValue :type "Float (single-precision)"))
  (bind (_returnvalue_roll _returnvalue_pitch _returnvalue_yaw) (`KismetMathLibrary.BreakRotator` (`self.GetControlRotation`)))
  (bind _yawlimit (`self.YawLimit`))
  (bind _returnvalue (* _yawlimit -1.0))
  (bind _returnvalue_2 (select `bool` (>= _returnvalue_yaw 180.0) :`false` _returnvalue_yaw :`true` (- _returnvalue_yaw 360.0)))
  (bind _binputenabled (`self.GetCurrentWeaponInputEnabled`))
  (if _binputenabled
    (`self.AddControllerYawInput` (`KismetMathLibrary.FClamp` AxisValue (`KismetMathLibrary.FClamp` (- _returnvalue _returnvalue_2) _returnvalue 0.0) (`KismetMathLibrary.FClamp` (- _yawlimit _returnvalue_2) 0.0 _yawlimit)))))

(event `InputAction|Fire`
  (params (Key :type "Key Structure" :default "AnyKey"))
  (bind _currentweapon (`SQPawnInventoryComponent.CurrentWeapon` (`self.GetVehicleInventory`)))
  (:`Pressed`
    (`SQEquipableItem.BeginUse` _currentweapon))
  (:`Released`
    (`SQEquipableItem.EndUse` _currentweapon)))

(fn `Get1PAttachComponent`
  (returns (ReturnValue :type "SceneComponent Object Reference"))
  (return (`self.GunAttachPoint`)))

(fn `Get3PAttachComponent`
  (returns (ReturnValue :type "SceneComponent Object Reference"))
  (return (`self.GunAttachPoint`)))

(fn `GetADSCameraLocationComponent`
  (returns (ReturnValue :type "SceneComponent Object Reference"))
  (return (`self.ADSCameraPosition`)))

(fn `GetCurrentWeaponInputEnabled`
  (returns (bInputEnabled :type Boolean))
  (bind _sqvehicleinventory (`self.SQVehicleInventory`)
    (:`then`
      (bind _assqvehicle_weapon (cast `SQVehicleWeapon` (`SQPawnInventoryComponent.CurrentWeapon` _sqvehicleinventory))
        (:`then`
          (if (`SQVehicleWeapon.bInputEnabled` _assqvehicle_weapon)
            (bind _returnvalue (`self.IsSoldierAlive`))
            (if _returnvalue
              (return true)
              (else
                (return false)))
            (else
              (return false))))
        (:`CastFailed`
          (return false))))
    (:`else`
      (return false))))

(fn `GetDefaultCameraLocationComponent`
  (returns (ReturnValue :type "SceneComponent Object Reference"))
  (return (`self.DefaultCameraPosition`)))

(fn `GetMasterPoseComponent`
  (returns (ReturnValue :type "SkinnedMeshComponent Object Reference"))
  (return null))

(fn `GetSoldierAttachComponent`
  (returns (ReturnValue :type "SceneComponent Object Reference"))
  (return (`SQVehicle.VehicleMesh` (`self.GetVehicle`))))

(fn `GetWeaponAttachComponent`
  (returns (ReturnValue :type "SceneComponent Object Reference"))
  (return (`self.GunAttachPoint`)))

(fn `IsCurrentWeaponInputEnabled`
  (returns (bInputEnabled :type Boolean))
  (bind _sqvehicleinventory (`self.SQVehicleInventory`)
    (:`then`
      (bind _assqvehicle_weapon (cast `SQVehicleWeapon` (`SQPawnInventoryComponent.CurrentWeapon` _sqvehicleinventory))
        (:`then`
          (if (`SQVehicleWeapon.bInputEnabled` _assqvehicle_weapon)
            (bind _returnvalue (`self.IsSoldierAlive`))
            (if _returnvalue
              (return true)
              (else
                (return false)))
            (else
              (return false))))
        (:`CastFailed`
          (return false))))
    (:`else`
      (return false))))

(fn `IsSoldierAlive`
  (returns (ReturnValue :type Boolean))
  (bind _currentweapon (`SQPawnInventoryComponent.CurrentWeapon` (`self.SQVehicleInventory`))
    (:`then`
      (bind _assqvehicle_weapon (cast `SQVehicleWeapon` _currentweapon)
        (:`then`
          (bind _returnvalue (`SQVehicleWeapon.GetSoldier` _assqvehicle_weapon))
          (`/Engine/EditorBlueprintResources/StandardMacros.IsValid` _returnvalue
            (:`Is Valid`
              (return (`SQSoldier.IsAlive` _returnvalue)))
            (:`Is Not Valid`
              (return false))))
        (:`CastFailed`
          (return false))))
    (:`else`
      (return false))))

(fn `UserConstructionScript`
  (set `SQStaticTurretMovementComponent.YawComponent` (`self.DefaultSceneRoot`) (`self.SQStaticTurretMovement`))
  (set `SQStaticTurretMovementComponent.PitchComponent` (`self.GunAttachPoint`) (`self.SQStaticTurretMovement`)))