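; Player-flyable Ka-52 attack helicopter vehicle, with coaxial rotors, animated doors, cockpit and external cameras, and missile armament.
; Gamepad and keyboard input feeds the HeliFM flight component, with keyboard throttle ramped on Tick while hovering.
; Tick also updates the cockpit screen from a ground trace, rearms at repair actors and spawns a wreck on destruction.
; Rotor meshes hide and swap bones for coning, and missiles fire from alternating launch points.
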(event `InputAxisKey|Gamepad_RightTriggerAxis`
  (params (AxisValue :type "Float (single-precision)"))
  (if (> AxisValue 0.0)
    (set `self.AxisLR` false)
    (if (not false)
      (`/Engine/EditorBlueprintResources/ActorMacros.Switch Has Authority`
        (:`Remote`
          (`/HelicopterTestMaps/HeliFM.InputControls` (`self.HeliFM`) 3 true AxisValue false))))))

(event `InputAxisKey|Gamepad_LeftTriggerAxis`
  (params (AxisValue :type "Float (single-precision)"))
  (if (> AxisValue 0.0)
    (set `self.AxisLR` true))
  (if (`self.IsUsingGamepad`)
    (if (`self.AxisLR`)
      (`/Engine/EditorBlueprintResources/ActorMacros.Switch Has Authority`
        (:`Remote`
          (`/HelicopterTestMaps/HeliFM.InputControls` (`self.HeliFM`) 3 false AxisValue false))))))

(event `Key|AnyKey`
  (params (Key :type "Key Structure" :default "AnyKey"))
  (:`Pressed`
    (if (`KismetInputLibrary.Key_IsGamepadKey` Key)
      (bind _output_get (set `self.IsUsingGamepad` true))
      (`self.ServerSetGamepad` _output_get))))

(event `ServerSetDestroyed`
  (params (Float :type Boolean))
  (set `self.DestroyedWatcher` Float))

(event `InputAxisKey|Gamepad_LeftY`
  (params (AxisValue :type "Float (single-precision)"))
  (if (`self.IsUsingGamepad`)
    (`/Engine/EditorBlueprintResources/ActorMacros.Switch Has Authority`
      (:`Remote`
        (`/HelicopterTestMaps/HeliFM.InputControls` (`self.HeliFM`) 0 false AxisValue false)))))

(event `InputAxisKey|Gamepad_RightY`
  (params (AxisValue :type "Float (single-precision)"))
  (if (`self.IsUsingGamepad`)
    (`/Engine/EditorBlueprintResources/ActorMacros.Switch Has Authority`
      (:`Remote`
        (`/HelicopterTestMaps/HeliFM.InputControls` (`self.HeliFM`) 1 false (* AxisValue 0.3) false)))))

(event `ServerSetGamepad`
  (params (Bool :type Boolean))
  (set `self.IsUsingGamepad` Bool))

(event `ServerSetFloatParam`
  (params (Float :type "Float (double-precision)"))
  (`AudioComponent.SetFloatParameter` (`self.EngineRPMAC`) "EngineSpeed" Float))

(event `InputAxisKey|Gamepad_RightX`
  (params (AxisValue :type "Float (single-precision)"))
  (if (`self.IsUsingGamepad`)
    (`/Engine/EditorBlueprintResources/ActorMacros.Switch Has Authority`
      (:`Remote`
        (`/HelicopterTestMaps/HeliFM.InputControls` (`self.HeliFM`) 2 false (* AxisValue 0.3) false)))))

(event `ServerIncEngine`
  (params (Int :type "Float (double-precision)") (Min :type "Float (double-precision)") (Bypass :type Boolean))
  (`self.IncEngine` Int Min Bypass))

(event `self.SpinRotor`
  (params (EngineSpeed :type "Float (single-precision)"))
  (bind _returnvalue (* EngineSpeed 0.04))
  (`SceneComponent.K2_AddLocalRotation` (`self.RotorMain`) (`KismetMathLibrary.MakeRotator` 0.0 0.0 _returnvalue) false false)
  (`SceneComponent.K2_AddLocalRotation` (`self.Ka52 Top`) (`KismetMathLibrary.MakeRotator` 0.0 0.0 (* _returnvalue -1.0)) false false))

(event `ServerSetHover`
  (params (NewParam :type Integer))
  (set `self.engineHover` NewParam))

(event `SpawnEffects`
  (params (`Emitter Class` :type "ParticleSystem Object Reference") (Location :type "Vector Structure") (Rotation :type "Rotator Structure") (Sound :type "SoundBase Object Reference"))
  (`GameplayStatics.SpawnEmitterAtLocation` `Emitter Class` Location Rotation)
  (`/Engine/EditorBlueprintResources/StandardMacros.IsValid` Sound
    (:`Is Valid`
      (`GameplayStatics.PlaySoundAtLocation` Sound Location))))

(event `ServerSetWarmup`
  (params (NewParam :type Boolean))
  (set `self.warmedUp` NewParam)
  (`SceneComponent.SetVisibility` (`self.ParticleSystem1`) NewParam false)
  (`SceneComponent.SetVisibility` (`self.ParticleSystem_0`) NewParam false))

(event `Fire Rocket`
  (bind _returnvalue (`SceneComponent.K2_GetComponentToWorld` (`self.Rocket2`)))
  (bind _returnvalue_2 (`SceneComponent.K2_GetComponentToWorld` (`self.Rocket1`)))
  (bind _returnvalue_3 (`SQVehicleSeatComponent.GetSeatPawn` (`|GetArrayItem` (`self.VehicleSeats`) 1)))
  (if (> (`self.HeliAmmo`) 0)
    (if (== (`self.CurrentRocket`) 0)
      (bind _returnvalue_4 (`|SpawnActorFromClass` "/HelicopterTestMaps/Ka52/Ka52Missile.Ka52Missile_C" _returnvalue_2 "Undefined" "OverrideRootScale" null _returnvalue_3))
      (set `/HelicopterTestMaps/Ka52/Ka52Missile.Helicopter` self _returnvalue_4)
      (set `self.CurrentRocket` 1)
      (`self.SpawnEffects` "/Game/Particles/Weapons/Anti-Tank/S5_BackBlast.S5_BackBlast" (.location _returnvalue_2) (`KismetMathLibrary.ComposeRotators` (.rotation _returnvalue_2) (struct :`Pitch` 90.0)) "/HelicopterTestMaps/Ka52/Sounds/SC_Ka52_MissileFire.SC_Ka52_MissileFire")
      (else
        (bind _returnvalue_5 (`|SpawnActorFromClass` "/HelicopterTestMaps/Ka52/Ka52Missile.Ka52Missile_C" _returnvalue "Undefined" "OverrideRootScale" null _returnvalue_3))
        (set `/HelicopterTestMaps/Ka52/Ka52Missile.Helicopter` self _returnvalue_5)
        (set `self.CurrentRocket` 0)
        (`self.SpawnEffects` "/Game/Particles/Weapons/Anti-Tank/S5_BackBlast.S5_BackBlast" (.location _returnvalue) (`KismetMathLibrary.ComposeRotators` (.rotation _returnvalue) (struct :`Pitch` 90.0)) "/HelicopterTestMaps/Ka52/Sounds/SC_Ka52_MissileFire.SC_Ka52_MissileFire")))
    (set `self.HeliAmmo` (- (`self.HeliAmmo`) 1))))

(event `SwitchRocket`
  (bind _sqvehicleinventory (`self.SQVehicleInventory`))
  (if (== (`SQPawnInventoryComponent.CurrentWeaponSlot` _sqvehicleinventory) 0)
    (`SQPawnInventoryComponent.SwitchWeapon` _sqvehicleinventory 1)
    (`SQEquipableItem.BeginUse` (`SQPawnInventoryComponent.CurrentWeapon` _sqvehicleinventory))
    (else
      (`SQPawnInventoryComponent.SwitchWeapon` _sqvehicleinventory 0))))

(event `Key|S`
  (params (Key :type "Key Structure" :default "AnyKey"))
  (:`Pressed`
    (`self.ServerSetS` true)
    (set `self.IsKeyAdjusting` (stale `ServerSetS` Bool) :!label _label)
    (set `self.ThrottleDirection` -1)
    (set `self.IsUsingGamepad` false))
  (:`Released`
    (`self.ServerSetS` false)))

(event `ServerSetS`
  (params (Bool :type Boolean))
  (goto _label))

(event `ServerSetControls`
  (params (Control :type Integer) (Bool :type Boolean))
  (switch `int` Control
    (:`Default`
      (set `self.EngineForward` Bool :!label _label_2))
    (:`0`
      (set `self.isDescending` Bool))
    (:`1`
      (set `self.turnRight` Bool))
    (:`2`
      (set `self.turnLeft` Bool))
    (:`3`
      (goto _label_2))))

(event `Key|D`
  (params (Key :type "Key Structure" :default "AnyKey"))
  (bind _helifm (`self.HeliFM`))
  (bind _returnvalue (`KismetMathLibrary.Conv_BoolToInt` (`self.InvertControls`)))
  (bind _returnvalue_2 (- 3 _returnvalue))
  (:`Pressed`
    (`/HelicopterTestMaps/HeliFM.InputControls` _helifm _returnvalue_2 true (- 1.0 (* _returnvalue 0.8)) true))
  (:`Released`
    (`/HelicopterTestMaps/HeliFM.InputControls` _helifm _returnvalue_2 true 0.0 true)
    (set `self.IsUsingGamepad` false :!label _label_3)))

(event `Key|A`
  (params (Key :type "Key Structure" :default "AnyKey"))
  (bind _helifm (`self.HeliFM`))
  (bind _returnvalue (`KismetMathLibrary.Conv_BoolToInt` (`self.InvertControls`)))
  (bind _returnvalue_2 (- 3 _returnvalue))
  (:`Pressed`
    (`/HelicopterTestMaps/HeliFM.InputControls` _helifm _returnvalue_2 false (- 1.0 (* _returnvalue 0.8)) true))
  (:`Released`
    (`/HelicopterTestMaps/HeliFM.InputControls` _helifm _returnvalue_2 false 0.0 true)
    (goto _label_3)))

(event `ConeProps`
  (params (Coning :type Boolean))
  (bind _rotormain (`self.RotorMain`))
  (bind _ka52_top (`self.Ka52 Top`))
  (if Coning
    (`SkinnedMeshComponent.HideBoneByName` _rotormain "blade_bottom_down" "PBO_None")
    (`SkinnedMeshComponent.UnHideBoneByName` _rotormain "blade_bottom_up")
    (`SkinnedMeshComponent.HideBoneByName` _ka52_top "blade_top_down" "PBO_None")
    (`SkinnedMeshComponent.UnHideBoneByName` _ka52_top "blade_top_up")
    (else
      (`SkinnedMeshComponent.HideBoneByName` _rotormain "blade_bottom_up" "PBO_None")
      (`SkinnedMeshComponent.UnHideBoneByName` _rotormain "blade_bottom_down")
      (`SkinnedMeshComponent.HideBoneByName` _ka52_top "blade_top_up" "PBO_None")
      (`SkinnedMeshComponent.UnHideBoneByName` _ka52_top "blade_top_down"))))

(event `ServerSetW`
  (params (Bool :type Boolean))
  (set `self.IsKeyAdjusting` Bool)
  (set `self.ThrottleDirection` 1)
  (set `self.IsUsingGamepad` false))

(event `Key|W`
  (params (Key :type "Key Structure" :default "AnyKey"))
  (:`Pressed`
    (`self.ServerSetW` true))
  (:`Released`
    (`self.ServerSetW` false)))

(event `ServerInputThrottle`
  (bind _keythrottle (`self.KeyThrottle`))
  (if (`/HelicopterTestMaps/HeliFM.IsHovering` (`self.HeliFM`))
    (if (not (`self.IsUsingGamepad`))
      (if (`self.IsKeyAdjusting`)
        (set `self.KeyThrottle` (`KismetMathLibrary.FClamp` (+ _keythrottle (* (`self.ThrottleDirection`) 0.03)) -1.0))
        (elif (not (== _keythrottle 0.0))
          (set `self.KeyThrottle` (`KismetMathLibrary.FClamp` (* (`KismetMathLibrary.SignOfFloat` _keythrottle) (- (`KismetMathLibrary.Abs` _keythrottle) 0.03)) -1.0))))
      (`/Engine/EditorBlueprintResources/ActorMacros.Switch Has Authority`
        (:`Authority`
          (`/HelicopterTestMaps/HeliFM.InputControls` (`self.HeliFM`) 0 false (`self.KeyThrottle`) false))))))

(event `Hide Bones`
  (bind _rotormain (`self.RotorMain`))
  (bind _ka52_top (`self.Ka52 Top`))
  (`SkinnedMeshComponent.HideBoneByName` _rotormain "rotor_top" "PBO_None")
  (`SkinnedMeshComponent.HideBoneByName` _rotormain "blade_top_up" "PBO_None")
  (`SkinnedMeshComponent.HideBoneByName` _rotormain "blade_top_down" "PBO_None")
  (`SkinnedMeshComponent.HideBoneByName` _rotormain "blade_bottom_up" "PBO_None")
  (`SkinnedMeshComponent.HideBoneByName` _ka52_top "rotor_bottom" "PBO_None")
  (`SkinnedMeshComponent.HideBoneByName` _ka52_top "blade_bottom_up" "PBO_None")
  (`SkinnedMeshComponent.HideBoneByName` _ka52_top "blade_bottom_down" "PBO_None")
  (`SkinnedMeshComponent.HideBoneByName` _ka52_top "blade_top_up" "PBO_None"))

(event `ToggleDoors`
  (params (State :type Boolean))
  (bind _doorstate (`self.DoorState`))
  (bind _vehiclemesh (`self.VehicleMesh`))
  ;[1 1 1] 1 = open, 0 =close
  (if State
    (if _doorstate
      _
      (else
        _))
    (`SkeletalMeshComponent.PlayAnimation` _vehiclemesh "/HelicopterTestMaps/Ka52/Model/Ka52_Armature_DoorsOpen.Ka52_Armature_DoorsOpen" false)
    (else
      (if _doorstate
        _
        (else
          _))
      (`SkeletalMeshComponent.PlayAnimation` _vehiclemesh "/HelicopterTestMaps/Ka52/Model/Ka52_Armature_DoorsClose.Ka52_Armature_DoorsClose" false))))

(event `InputAction|VehicleToggleEngine`
  (params (Key :type "Key Structure" :default "AnyKey"))
  (bind _helifm (`self.HeliFM`))
  (:`Pressed`
    (if (`self.bIsEngineActive`)
      (`/HelicopterTestMaps/HeliFM.StopEngine` _helifm)
      (`self.ServerToggleDoors` true)
      (`KismetSystemLibrary.Delay` 1.5)
      (`self.ServerSetCone` false)
      (elif (not (`/HelicopterTestMaps/HeliFM.StartingUp` _helifm))
        (`/HelicopterTestMaps/HeliFM.StartEngine` _helifm)
        (`self.ServerToggleDoors` false)
        (`KismetSystemLibrary.Delay` 3.0)
        (`SceneComponent.SetVisibility` (`self.ParticleSystem1`) true false)
        (`SceneComponent.SetVisibility` (`self.ParticleSystem_0`) true false)
        (`KismetSystemLibrary.Delay` 3.0)
        (`self.ServerSetCone` true)))))

(event `ServerToggleDoors`
  (params (State :type Boolean))
  (`self.ToggleDoors` State)
  (set `self.DoorState` State))

(event `self.ReceiveTick`
  (params (DeltaSeconds :type "Float (single-precision)"))
  (bind (_returnvalue_x _returnvalue_y) (`KismetMathLibrary.BreakVector` (`self.GetVelocity`)))
  (bind (_returnvalue_roll _returnvalue_pitch) (`KismetMathLibrary.BreakRotator` (`self.K2_GetActorRotation`)))
  (bind _returnvalue (`SceneComponent.K2_GetComponentLocation` (`self.VehicleMesh`)))
  (bind _returnvalue_2 (+ _returnvalue (0.0 0.0 5.0)))
  (if (`self.bHasBeenDestroyed`)
    (if (not (`self.DestroyedWatcher`))
      (`self.SpawnWreck` (`self.GetVelocity`))
      (set `self.DestroyedWatcher` true)
      (`self.ServerSetDestroyed` true))
    (else
      (if (>= (`KismetArrayLibrary.Array_LastIndex` (`self.GetOverlappingActors` "/Game/Gameplay/Deployables/BP_vehicle_repair.BP_vehicle_repair_C")) 0)
        (`/Engine/EditorBlueprintResources/ActorMacros.Switch Has Authority`
          (:`Authority`
            (`self.CustomRearm` self))
          (:`Remote`
            _)))
      (bind _aska_52screen_actor (cast `/HelicopterTestMaps/Ka52/Ka52ScreenActor` (`ChildActorComponent.ChildActor` (`self.BlackhawkScreen`))))
      (bind _outhit (`KismetSystemLibrary.LineTraceSingle` _returnvalue_2 (+ _returnvalue (0.0 0.0 -10000.0)) "TraceTypeQuery1"))
      (bind (_bblockinghit _binitialoverlap _time _location) (`GameplayStatics.BreakHitResult` _outhit))
      (bind _z (.z (- _location _returnvalue_2)))
      (set `self.Altitude` _z)
      (set `self.DustTransform` (`KismetMathLibrary.Conv_VectorToTransform` _location))
      (`/HelicopterTestMaps/Ka52/Ka52ScreenActor.UpdatePitchWidget` _aska_52screen_actor (`KismetMathLibrary.FClamp` _returnvalue_pitch -50.0 50.0) _returnvalue_roll (* (`KismetMathLibrary.FTrunc` _z) -1) (`/HelicopterTestMaps/HeliFM.Throttle` (`self.HeliFM`)) (`KismetMathLibrary.VSize` (`KismetMathLibrary.MakeVector` _returnvalue_x _returnvalue_y)) (`self.InvertControls`) (`self.HeliAmmo`) (`self.DeployedRopes`) (`self.TurretYawAngle`))
      (if (not (`self.IsUsingGamepad`))
        (`self.ServerInputThrottle`)))))

(event `ServerSetCone`
  (params (Coning :type Boolean))
  (`self.ConeProps` Coning))

(event `self.ReceiveBeginPlay`
  (`parent.ReceiveBeginPlay`)
  (`/Engine/EditorBlueprintResources/ActorMacros.Switch Has Authority`
    (:`Authority`
      (`self.ServerToggleDoors` true))
    (:`Remote`
      (if (`self.DoorState`)
        (`self.ToggleDoors` true))))
  (add `self.OnVehicleRepairEvent` (delegate `OnVehicleRepairEvent_Event_0`))
  (`self.Hide Bones`)
  (`ActorComponent.Activate` (`self.Camera`) false)
  (`ActorComponent.Deactivate` (`self.ExternalCamera`))
  (if (not (`self.HasRockets`))
    (`SkinnedMeshComponent.HideBoneByName` (`self.VehicleMesh`) "Missiles" "PBO_None")))

(event `OnVehicleRepairEvent_Event_0` :!signature `self.OnVehicleRepairEvent`
  (params (Vehicle :type "SQVehicle Object Reference"))
  (`KismetSystemLibrary.Delay` 1.0)
  (`self.CustomRearm` Vehicle))

(event `CustomRearm`
  (params (NewParam :type "SQVehicle Object Reference"))
  (bind _returnvalue (`self.GetVehicleInventory` NewParam))
  (`/Engine/EditorBlueprintResources/StandardMacros.DoOnce` false :!label _label_4
    (:`Completed`
      (set `self.HeliAmmo` (`KismetMathLibrary.Clamp` (+ (`self.HeliAmmo`) 1) 0 14))
      (bind _aska_52_gun (cast `/HelicopterTestMaps/Ka52/Ka52_Gun` (`ChildActorComponent.ChildActor` (`self.Ka52_30mm`))))
      (set `/HelicopterTestMaps/Ka52/Ka52_Gun.30Ammo` (`KismetMathLibrary.Clamp` (+ (`/HelicopterTestMaps/Ka52/Ka52_Gun.30Ammo` _aska_52_gun) 20) 0 200) _aska_52_gun)
      (`KismetArrayLibrary.Array_Clear` (`SQPawnInventoryComponent.TestInventory` _returnvalue))
      (`KismetArrayLibrary.Array_Clear` (`SQVehicleInventoryComponent.Weapons` _returnvalue))
      (`SQPawnInventoryComponent.RemoveItemClassFromInventory` _returnvalue "/HelicopterTestMaps/Ka52/BP_UB32_Ka52.BP_UB32_Ka52_C")
      (bind _returnvalue_2 (`SQPawnInventoryComponent.AddGroupToInventory` _returnvalue))
      (`SQPawnInventoryComponent.InsertItemIntoInventory` _returnvalue 0 (make `SQInventoryData` "/HelicopterTestMaps/Ka52/BP_UB32_Ka52.BP_UB32_Ka52_C") _returnvalue_2)
      (bind _returnvalue_3 (`SQPawnInventoryComponent.AddGroupToInventory` _returnvalue))
      (`SQPawnInventoryComponent.InsertItemIntoInventory` _returnvalue 1 (make `SQInventoryData` "/HelicopterTestMaps/Ka52/BP_UB32_Ka52.BP_UB32_Ka52_C") _returnvalue_3)
      (`KismetSystemLibrary.Delay` 12.0)
      (goto _label_4 :!via `Reset`))))

(event `InputAction|ToggleView`
  (params (Key :type "Key Structure" :default "AnyKey"))
  (bind _camera (`self.Camera`))
  (bind _externalcamera (`self.ExternalCamera`))
  (:`Pressed`
    (if (`SQBlueprintLibrary.IsShippingBuild`)
      _
      (else
        _))
    (if (`ActorComponent.IsActive` (`self.Camera`))
      (`ActorComponent.Deactivate` _camera)
      (`ActorComponent.Activate` _externalcamera false)
      (else
        (`ActorComponent.Activate` _camera false)
        (`ActorComponent.Deactivate` _externalcamera)))))

(event `self.VehicleMesh.OnComponentHit`
  (params (HitComponent :type "PrimitiveComponent Object Reference") (OtherActor :type "Actor Object Reference") (OtherComp :type "PrimitiveComponent Object Reference") (NormalImpulse :type "Vector Structure") (Hit :type "HitResult Structure (by ref)"))
  (bind _returnvalue (`KismetMathLibrary.VSize` NormalImpulse))
  (if (> _returnvalue (`self.minImpactSpeed_0`))
    (`GameplayStatics.ApplyDamage` self (* 100 (/ _returnvalue (`self.minImpactSpeed_0`))) null null "/Script/Squad.SQBurningDamage")))

(event `SpawnWreck`
  (params (Vel :type "Vector Structure"))
  (bind _returnvalue (`|SpawnActorFromClass` "/HelicopterTestMaps/Ka52/Wreck/KA52_Wreckage3.KA52_Wreckage3_C" (`self.GetTransform`) "AlwaysSpawn" "OverrideRootScale" null "Team_Neutral"))
  (`PrimitiveComponent.AddImpulse` (`SQVehicle.VehicleMesh` _returnvalue) Vel "None" true))

(event `InputAxisKey|MouseY`
  (params (AxisValue :type "Float (single-precision)"))
  (bind _pitchlimit (`self.PitchLimit`))
  (bind _returnvalue (* (`self.PitchLimit`) -1.0))
  (bind (_relativerotation_roll _relativerotation_pitch) (`KismetMathLibrary.BreakRotator` (`SceneComponent.RelativeRotation` (`self.Camera`))))
  (bind _returnvalue_2 (select `bool` (>= _relativerotation_pitch 180.0) :`false` _relativerotation_pitch :`true` (- _relativerotation_pitch 360.0)))
  ;[1 1 1] Driver Head Rotation
  (if (`self.Free Looking`)
    (`SceneComponent.K2_AddRelativeRotation` (`self.Camera`) (`KismetMathLibrary.MakeRotator` 0.0 (`KismetMathLibrary.FClamp` AxisValue (`KismetMathLibrary.FClamp` (- _returnvalue _returnvalue_2) _returnvalue 0.0) (`KismetMathLibrary.FClamp` (- _pitchlimit _returnvalue_2) 0.0 _pitchlimit))) false false)))

(event `InputAxis|Turn`
  (params (AxisValue :type "Float (single-precision)"))
  (bind _camera (`self.Camera`))
  (bind _yawlimit (`self.YawLimit`))
  (bind _returnvalue (* _yawlimit -1.0))
  (bind (_relativerotation_roll _relativerotation_pitch _relativerotation_yaw) (`KismetMathLibrary.BreakRotator` (`SceneComponent.RelativeRotation` (`self.Camera`))))
  (bind _returnvalue_2 (select `bool` (>= _relativerotation_yaw 180.0) :`false` _relativerotation_yaw :`true` (- _relativerotation_yaw 360.0)))
  ;[1 1 1] Driver Head Rotation
  (if (`self.Free Looking`)
    (`SceneComponent.K2_AddRelativeRotation` _camera (`KismetMathLibrary.MakeRotator` 0.0 0.0 (`KismetMathLibrary.FClamp` AxisValue (`KismetMathLibrary.FClamp` (- _returnvalue _returnvalue_2) _returnvalue 0.0) (`KismetMathLibrary.FClamp` (- _yawlimit _returnvalue_2) 0.0 _yawlimit))) false false)
    (else
      (`SceneComponent.K2_SetRelativeRotation` :`self` _camera))))

(fn `IncEngine`
  (params (Int :type "Float (double-precision)") (Min :type "Float (double-precision)") (WarmupBypass :type Boolean))
  (bind _enginepower (`self.EnginePower`))
  (if (> 0.0 Int)
    _
    (else
      _))
  (if (`self.warmedUp`)
    (set `self.EnginePower` (`KismetMathLibrary.FClamp` (+ (`self.EnginePower`) Int) Min 8.0) :!label _label)
    (`self.ServerSetFloatParam` _enginepower)
    (`AudioComponent.SetFloatParameter` (`self.EngineSpeedAC`) "EngineSpeed" _enginepower)
    (`AudioComponent.SetFloatParameter` (`self.EngineRPMAC`) "EngineSpeed" _enginepower)
    (elif WarmupBypass
      (goto _label))))

(fn `SpawnWreckage`
  (params (Velocity :type "Vector Structure"))
  (bind _returnvalue (`|SpawnActorFromClass` "/HelicopterTestMaps/BlackhawkH_Backup/wreckage/BlackhawkWreckage.BlackhawkWreckage_C" (`self.GetTransform`) "AlwaysSpawn" "OverrideRootScale"))
  (`self.K2_DestroyActor`)
  (`PrimitiveComponent.AddImpulse` (`/HelicopterTestMaps/BlackhawkH_Backup/wreckage/BlackhawkWreckage.SkeletalMesh` _returnvalue) Velocity "None" true))

(fn `ToggleCustomPas`)

(fn `UserConstructionScript`
  (bind _rotormain (`self.RotorMain`))
  (bind _ka52_top (`self.Ka52 Top`))
  (`parent.UserConstructionScript`)
  (`SkinnedMeshComponent.HideBoneByName` _rotormain "rotor_top" "PBO_None")
  (`SkinnedMeshComponent.HideBoneByName` _rotormain "blade_top_up" "PBO_None")
  (`SkinnedMeshComponent.HideBoneByName` _rotormain "blade_top_down" "PBO_None")
  (`SkinnedMeshComponent.HideBoneByName` _rotormain "blade_bottom_up" "PBO_None")
  (`SkinnedMeshComponent.HideBoneByName` _ka52_top "rotor_bottom" "PBO_None")
  (`SkinnedMeshComponent.HideBoneByName` _ka52_top "blade_bottom_up" "PBO_None")
  (`SkinnedMeshComponent.HideBoneByName` _ka52_top "blade_bottom_down" "PBO_None")
  (`SkinnedMeshComponent.HideBoneByName` _ka52_top "blade_top_up" "PBO_None"))