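; Ka-52 30mm high-explosive cannon projectile (green variant) that detonates on impact.
; On Hit it runs the parent handler, then CustomImpact spawns a metal-impact particle effect aligned to the surface normal.
; CustomImpact then applies radial damage with falloff slightly above the actor's location, plays the impact sound and destroys the projectile.
; OnImpact only forwards to the parent.
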(event `CustomImpact`
  (params (Loc :type "Vector Structure") (Rot :type "Rotator Structure"))
  (bind _returnvalue (`self.K2_GetActorLocation`))
  (`GameplayStatics.SpawnEmitterAtLocation` "/Game/Particles/Impacts/Auto_Cannons/30mm_HE/bhit_30mm_HE_Metal.bhit_30mm_HE_Metal" Loc Rot)
  (`GameplayStatics.ApplyRadialDamageWithFalloff` :`BaseDamage` (`self.ExplosiveBaseDamage`) :`MinimumDamage` (`self.ExplosiveMinimumDamage`) :`Origin` (+ _returnvalue (0.0 0.0 20.0)) :`DamageInnerRadius` (`self.ExplosiveDamageInnerRadius`) :`DamageOuterRadius` (`self.ExplosiveDamageOuterRadius`) :`DamageFalloff` 1.0 :`DamageTypeClass` (`self.DamageTypeToApply`) :`DamageCauser` self :`InstigatedByController` (`self.GetInstigatorController`))
  (`GameplayStatics.PlaySoundAtLocation` "/Game/Audio/Impacts/Bullethits/30mm/HE/Bhit_30mm_HE_default_Cue.Bhit_30mm_HE_default_Cue" _returnvalue)
  (`self.K2_DestroyActor`))

(event `self.ReceiveHit`
  (params (MyComp :type "PrimitiveComponent Object Reference") (Other :type "Actor Object Reference") (OtherComp :type "PrimitiveComponent Object Reference") (bSelfMoved :type Boolean) (HitLocation :type "Vector Structure") (HitNormal :type "Vector Structure") (NormalImpulse :type "Vector Structure") (Hit :type "HitResult Structure (by ref)"))
  (`parent.ReceiveHit` MyComp Other OtherComp bSelfMoved HitLocation HitNormal NormalImpulse Hit)
  (`self.CustomImpact` HitLocation (`KismetMathLibrary.Conv_VectorToRotator` HitNormal)))

(event `self.OnImpact`
  (params (SelfActor :type "Actor Object Reference") (OtherActor :type "Actor Object Reference") (NormalImpulse :type "Vector Structure") (Hit :type "HitResult Structure (by ref)"))
  (`parent.OnImpact` SelfActor OtherActor NormalImpulse Hit))

(fn `UserConstructionScript`)