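; UB-32 rocket pod weapon for the Ka-52 helicopter, with heat-based overheating.
; Firing adds temperature, plays backblast shockwave, muzzle and blast effects, and calls SwitchRocket on the parent Ka-52 on remote clients.
; Temperature triggers set the overheat flag and drive three stages of lazily spawned, reused particles and looping sounds.
; Seat enter/exit runs montage helpers that cast to BP_EmplacedM2, though entry passes them no montages.
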(event `self.SQTemperature.OnTemperatureIncrementEvent`
  (params (TriggeringComponent :type "SQTemperatureComponent Object Reference") (TriggeringTemp :type "Float (single-precision)") (bIsLowerTrigger :type Boolean))
  (`|ExecutionSequence`
    (:`then_0`
      (`self.Set Overheat Variable` bIsLowerTrigger TriggeringTemp))
    (:`then_1`
      (`self.Setup Overheat Effect` bIsLowerTrigger TriggeringTemp))))

(event `self.BlueprintOnFire`
  (params (Origin :type "Vector Structure"))
  (bind _shockwave1p (`self.Shockwave1p`))
  (bind _returnvalue (`SceneComponent.K2_GetComponentLocation` (`self.Mesh3P`)))
  (`parent.BlueprintOnFire` Origin)
  (`SQTemperatureComponent.AdjustTemperature` (`self.SQTemperature`) 1.0 null)
  (`/Engine/EditorBlueprintResources/StandardMacros.Can Execute Cosmetic Events`
    (:`True`
      (bind _asbp_back_blast_shock_wave (cast `/Game/Blueprints/Effects/BP_BackBlastShockWave` (select `bool` (`self.IsFirstPersonViewTarget`) :`false` (`ChildActorComponent.ChildActor` (`self.Shockwave3p`)) :`true` (`ChildActorComponent.ChildActor` _shockwave1p) :!type "Object Object Reference")))
      (`/Game/Blueprints/Effects/BP_Shockwave.Explode` _asbp_back_blast_shock_wave (`self.Instigator`))
      (`GameplayStatics.SpawnEmitterAtLocation` self (`self.BackblastEffect3P`) _returnvalue (`SceneComponent.K2_GetComponentRotation` _shockwave1p))
      (`GameplayStatics.SpawnEmitterAtLocation` "/Game/Particles/Weapons/Anti-Tank/Muzzleflash_S5.Muzzleflash_S5" _returnvalue (`SceneComponent.K2_GetComponentRotation` (`self.Muzzle`)))
      (`SQBlastComponent.FireBlast` (`self.SQBlast`))
      (bind _asbp_ka_52 (cast `/HelicopterTestMaps/Ka52/BP_Ka52` (`self.GetAttachParentActor`)))
      (`/Engine/EditorBlueprintResources/ActorMacros.Switch Has Authority`
        (:`Remote`
          (`/HelicopterTestMaps/Ka52/BP_Ka52.SwitchRocket` _asbp_ka_52))))))

(event `self.BlueprintOnReload`
  (`parent.BlueprintOnReload`))

(event `self.SoldierEntersVehicle`
  (params (Soldier :type "SQSoldier Object Reference"))
  (set `self.bInputEnabled` false)
  (`parent.SoldierEntersVehicle` Soldier)
  (if (`self.IsReloading`)
    (`self.ResumeAnimations` null)
    (else
      (`/Engine/EditorBlueprintResources/StandardMacros.IsValid` Soldier
        (:`Is Valid`
          (bind (_tripodanimtime _weaponanimtime) (`self.PlayAnimations` null null null Soldier))
          (`KismetSystemLibrary.Delay` _weaponanimtime)
          (set `self.bInputEnabled` true))))))

(event `self.SoldierLeavesVehicle`
  (params (Soldier :type "SQSoldier Object Reference"))
  (`parent.SoldierLeavesVehicle` Soldier)
  (`/Engine/EditorBlueprintResources/StandardMacros.IsValid` Soldier
    (:`Is Valid`
      (`self.StopAnimations` Soldier))))

(fn `PlayAnimations`
  (params (TripodAnim :type "AnimMontage Object Reference") (WeaponAnim :type "AnimMontage Object Reference") (SoldierAnim :type "AnimMontage Object Reference") (Soldier :type "SQSoldier Object Reference"))
  (returns (TripodAnimTime :type "Float (double-precision)") (WeaponAnimTime :type "Float (double-precision)") (SoldierAnimTime :type "Float (double-precision)"))
  (locals (TripodPlayTime :type "Float (double-precision)") (WeaponPlayTime :type "Float (double-precision)") (SoliderPlayTime :type "Float (double-precision)") (LocalSoldier :type "SQSoldier Object Reference"))
  (bind _returnvalue (`self.GetOwnerPawn`))
  (`/Engine/EditorBlueprintResources/StandardMacros.Can Execute Cosmetic Events`
    (:`True`
      ;[1 1 1] Set Local Soldier
      (`/Engine/EditorBlueprintResources/StandardMacros.IsValid` Soldier
        (:`Is Valid`
          (set `local.LocalSoldier` Soldier))
        (:`Is Not Valid`
          (set `local.LocalSoldier` (`self.GetSoldier`))))
      (`|ExecutionSequence`
        (:`then_0`
          ;[1 1 1] Tripod Animation
          (`/Engine/EditorBlueprintResources/StandardMacros.IsValid` TripodAnim
            (:`Is Valid`
              (`/Engine/EditorBlueprintResources/StandardMacros.IsValid` _returnvalue
                (:`Is Valid`
                  (bind _asbp_emplaced_m2 (cast `/Game/Vehicles/Emplaced50cal/BP_EmplacedM2` _returnvalue))
                  (`AnimInstance.Montage_Play` (`SkeletalMeshComponent.GetAnimInstance` (`SQVehicle.VehicleMesh` _asbp_emplaced_m2)) TripodAnim 1.0 "MontageLength" 0.0)
                  (bind _returnvalue_2 (`AnimSequenceBase.GetPlayLength` TripodAnim))
                  (set `local.TripodPlayTime` _returnvalue_2))))))
        (:`then_1`
          ;[1 1 1] Weapon Animation
          (`/Engine/EditorBlueprintResources/StandardMacros.IsValid` WeaponAnim
            (:`Is Valid`
              (`AnimInstance.Montage_Play` (`SkeletalMeshComponent.GetAnimInstance` (`self.Mesh3P`)) WeaponAnim 1.0 "MontageLength" 0.0)
              (bind _returnvalue_3 (`AnimSequenceBase.GetPlayLength` WeaponAnim))
              (set `local.WeaponPlayTime` _returnvalue_3))))
        (:`then_2`
          ;[1 1 1] Soldier Animation
          (`/Engine/EditorBlueprintResources/StandardMacros.IsValid` SoldierAnim
            (:`Is Valid`
              (`/Engine/EditorBlueprintResources/StandardMacros.IsValid` (`local.LocalSoldier`)
                (:`Is Valid`
                  (`Character.PlayAnimMontage` (`local.LocalSoldier`) SoldierAnim 1.0 "None")
                  (bind _returnvalue_4 (`AnimSequenceBase.GetPlayLength` SoldierAnim))
                  (set `local.SoliderPlayTime` _returnvalue_4))))))
        (:`then_3`
          (return (`local.TripodPlayTime`) (`local.WeaponPlayTime`) (`local.SoliderPlayTime`)))))
    (:`False`
      (return 0.0 0.0 0.0) ; Server doesn't play animations
    )))

(fn `ResumeAnimations`
  (params (TripodAnim :type "AnimMontage Object Reference") (WeaponAnim :type "AnimMontage Object Reference") (SoldierAnim :type "AnimMontage Object Reference"))
  (bind _returnvalue (`self.GetOwnerPawn`))
  (bind _returnvalue_2 (`self.GetSoldier`))
  (bind _returnvalue_3 (`SkeletalMeshComponent.GetAnimInstance` (`self.Mesh3P`)))
  (`|ExecutionSequence`
    (:`then_0`
      (`/Engine/EditorBlueprintResources/StandardMacros.IsValid` TripodAnim
        (:`Is Valid`
          (`/Engine/EditorBlueprintResources/StandardMacros.IsValid` _returnvalue
            (:`Is Valid`
              (bind _asbp_emplaced_m2 (cast `/Game/Vehicles/Emplaced50cal/BP_EmplacedM2` _returnvalue))
              (`AnimInstance.Montage_Play` (`SkeletalMeshComponent.GetAnimInstance` (`SQVehicle.VehicleMesh` _asbp_emplaced_m2)) TripodAnim 1.0 "MontageLength" 0.0))))))
    (:`then_1`
      (`/Engine/EditorBlueprintResources/StandardMacros.IsValid` WeaponAnim
        (:`Is Valid`
          (`AnimInstance.Montage_Play` _returnvalue_3 WeaponAnim 1.0 "MontageLength" 0.0)
          (`AnimInstance.Montage_JumpToSection` _returnvalue_3 (`self.Mesh3PReturnSection`) null))))
    (:`then_2`
      (`/Engine/EditorBlueprintResources/StandardMacros.IsValid` SoldierAnim
        (:`Is Valid`
          (`/Engine/EditorBlueprintResources/StandardMacros.IsValid` _returnvalue_2
            (:`Is Valid`
              (`Character.PlayAnimMontage` _returnvalue_2 SoldierAnim 1.0 (`self.SoldierMeshReturnSection`)))))))))

(fn `StopAnimations`
  (params (Soldier :type "SQSoldier Object Reference"))
  (bind _returnvalue (`self.GetOwnerPawn`))
  (bind _returnvalue_2 (`SkeletalMeshComponent.GetAnimInstance` (`self.Mesh3P`)))
  (bind _returnvalue_3 (`SkeletalMeshComponent.GetAnimInstance` (`Character.Mesh` Soldier)))
  (`|ExecutionSequence`
    (:`then_0`
      (`/Engine/EditorBlueprintResources/StandardMacros.IsValid` _returnvalue
        (:`Is Valid`
          (bind _asbp_emplaced_m2 (cast `/Game/Vehicles/Emplaced50cal/BP_EmplacedM2` _returnvalue))
          (bind _returnvalue_4 (`SkeletalMeshComponent.GetAnimInstance` (`SQVehicle.VehicleMesh` _asbp_emplaced_m2)))
          (`/Engine/EditorBlueprintResources/StandardMacros.IsValid` _returnvalue_4
            (:`Is Valid`
              (`AnimInstance.Montage_Pause` _returnvalue_4 null))))))
    (:`then_1`
      (`/Engine/EditorBlueprintResources/StandardMacros.IsValid` _returnvalue_2
        (:`Is Valid`
          (`AnimInstance.Montage_Pause` _returnvalue_2 null)
          (set `self.Mesh3PReturnSection` (`AnimInstance.Montage_GetCurrentSection` _returnvalue_2 null)))))
    (:`then_2`
      (`/Engine/EditorBlueprintResources/StandardMacros.IsValid` Soldier
        (:`Is Valid`
          (set `self.SoldierMeshReturnSection` (`AnimInstance.Montage_GetCurrentSection` _returnvalue_3 null))
          (`Character.StopAnimMontage` Soldier null)
          (bind _assqsoldier_anim_instance (cast `SQSoldierAnimInstance` _returnvalue_3))
          (set `SQSoldierAnimInstance.RightHandIKAlpha` 0.0 _assqsoldier_anim_instance)
          (set `SQSoldierAnimInstance.LeftHandIKAlpha` 0.0 _assqsoldier_anim_instance))))))

(fn `UserConstructionScript`)