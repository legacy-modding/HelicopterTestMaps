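; Projectile Blueprint for the Ka-52's 30mm high-explosive round, extending a parent projectile's impact behavior.
; On impact it calls the parent handler, then CustomImpact spawns a metal-hit particle effect oriented to the surface normal.
; CustomImpact also applies radial damage with falloff, centered slightly above the projectile and credited to its instigator.
; BeginPlay and Hit events only print debug strings.
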(event `CustomImpact`
  (params (Loc :type "Vector Structure") (Rot :type "Rotator Structure"))
  (`GameplayStatics.SpawnEmitterAtLocation` "/Game/Particles/Impacts/Auto_Cannons/30mm_HE/bhit_30mm_HE_Metal.bhit_30mm_HE_Metal" Loc Rot)
  (`GameplayStatics.ApplyRadialDamageWithFalloff` :`BaseDamage` (`self.ExplosiveBaseDamage`) :`MinimumDamage` (`self.ExplosiveMinimumDamage`) :`Origin` (+ (`self.K2_GetActorLocation`) (0.0 0.0 20.0)) :`DamageInnerRadius` (`self.ExplosiveDamageInnerRadius`) :`DamageOuterRadius` (`self.ExplosiveDamageOuterRadius`) :`DamageFalloff` 1.0 :`DamageTypeClass` (`self.DamageTypeToApply`) :`DamageCauser` self :`InstigatedByController` (`self.GetInstigatorController`)))

(event `self.OnImpact`
  (params (SelfActor :type "Actor Object Reference") (OtherActor :type "Actor Object Reference") (NormalImpulse :type "Vector Structure") (Hit :type "HitResult Structure (by ref)"))
  (bind (_bblockinghit _binitialoverlap _time _location _impactpoint _normal) (`GameplayStatics.BreakHitResult` Hit))
  (`parent.OnImpact` SelfActor OtherActor NormalImpulse Hit)
  (`self.CustomImpact` _location (`KismetMathLibrary.Conv_VectorToRotator` _normal)))

(event `self.ReceiveBeginPlay`
  (`KismetSystemLibrary.PrintString` "Begin"))

(event `self.ReceiveHit`
  (params (MyComp :type "PrimitiveComponent Object Reference") (Other :type "Actor Object Reference") (OtherComp :type "PrimitiveComponent Object Reference") (bSelfMoved :type Boolean) (HitLocation :type "Vector Structure") (HitNormal :type "Vector Structure") (NormalImpulse :type "Vector Structure") (Hit :type "HitResult Structure (by ref)"))
  (`KismetSystemLibrary.PrintString` "Hit"))

(fn `UserConstructionScript`)