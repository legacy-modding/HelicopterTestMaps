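; Test plane Blueprint built around an EasyFM flight model component, with cockpit and external cameras.
; BeginPlay selects the main camera and, after a short delay, applies full throttle; ToggleView swaps cameras when world settings allow third-person driving.
; Input stores throttle, mouse pitch and A/D roll in variables, but the UpdateControls call that would feed them to EasyFM is disconnected, so they never reach it.
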(event `self.ReceiveTick`
  (params (DeltaSeconds :type "Float (single-precision)")))

(event `InputAction|ToggleView`
  (params (Key :type "Key Structure" :default "AnyKey"))
  (bind _externalcamera (`self.ExternalCamera`))
  (bind _camera (`self.Camera`))
  (:`Pressed`
    (bind _returnvalue (`SQBlueprintLibrary.GetWorldSettings`))
    (bind _assqworld_settings (cast `SQWorldSettings` _returnvalue))
    (if (`SQWorldSettings.bCanDriverSwitchTo3rdPerson` _assqworld_settings)
      (if (`ActorComponent.IsActive` (`self.Camera`))
        (`ActorComponent.Deactivate` _camera)
        (`ActorComponent.Activate` _externalcamera false)
        (else
          (`ActorComponent.Activate` _camera false)
          (`ActorComponent.Deactivate` _externalcamera))))))

(event `self.ReceiveBeginPlay`
  (`ActorComponent.Activate` (`self.Camera`) false)
  (`ActorComponent.Deactivate` (`self.ExternalCamera`))
  (`KismetSystemLibrary.Delay` 1.0)
  (`easyFM.SetThrottleInput` (`self.easyFM`) 1.0))

(event `Key|A`
  (params (Key :type "Key Structure" :default "AnyKey"))
  (bind (_controls_x _controls_y) (`KismetMathLibrary.BreakVector` (`self.Controls`)))
  (:`Pressed`
    (set `self.Controls` (`KismetMathLibrary.MakeVector` _controls_x _controls_y -1.0)))
  (:`Released`
    (set `self.Controls` (0.0 0.0 0.0))))

(event `InputAxis|MoveForward`
  (params (AxisValue :type "Float (single-precision)"))
  (set `self.Throttle` (`KismetMathLibrary.FClamp` (+ (`self.Throttle`) (* AxisValue (`GameplayStatics.GetWorldDeltaSeconds`) 0.33)))))

(event `Key|D`
  (params (Key :type "Key Structure" :default "AnyKey"))
  (bind (_controls_x _controls_y) (`KismetMathLibrary.BreakVector` (`self.Controls`)))
  (:`Pressed`
    (set `self.Controls` (`KismetMathLibrary.MakeVector` _controls_x _controls_y 1.0)))
  (:`Released`
    (set `self.Controls` (0.0 0.0 0.0))))

(event `InputAxisKey|MouseX`
  (params (AxisValue :type "Float (single-precision)")))

(event `InputAxisKey|MouseY`
  (params (AxisValue :type "Float (single-precision)"))
  (bind (_controls_x _controls_y _controls_z) (`KismetMathLibrary.BreakVector` (`self.Controls`)))
  (set `self.Controls` (`KismetMathLibrary.MakeVector` (`KismetMathLibrary.FClamp` (+ _controls_x (* AxisValue 0.025)) -1.0) _controls_y _controls_z)))

(fn `Update Controls`
  (params (Throttle :type "Float (double-precision)") (Yaw :type "Float (double-precision)") (Roll :type "Float (double-precision)") (Pitch :type "Float (double-precision)"))
  (bind _easyfm (`self.easyFM`))
  (`easyFM.SetPitchInput` _easyfm Pitch)
  (`easyFM.SetYawInput` _easyfm Yaw)
  (`easyFM.SetRollInput` _easyfm Roll)
  (`easyFM.SetThrottleInput` _easyfm Throttle)
  (return))

(fn `UserConstructionScript`)