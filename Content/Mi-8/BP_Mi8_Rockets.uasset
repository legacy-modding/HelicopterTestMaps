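; Mi-8 helicopter rockets Blueprint that manages two UB-32 rocket weapons and their rearming.
; SwitchRocket toggles between inventory slots 0 and 1, immediately starting use of the weapon when moving to slot 1.
; Rearm triggers from an authority-only Tick check for overlapping repair actors, or one second after a vehicle repair event.
; CustomRearm clears and rebuilds the inventory with both pods, throttled by a DoOnce that resets after five seconds.
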(event `self.ReceiveTick`
  (params (DeltaSeconds :type "Float (single-precision)"))
  (`parent.ReceiveTick` DeltaSeconds)
  (if (>= (`KismetArrayLibrary.Array_LastIndex` (`self.GetOverlappingActors` "/Game/Gameplay/Deployables/BP_vehicle_repair.BP_vehicle_repair_C")) 0)
    (`/Engine/EditorBlueprintResources/ActorMacros.Switch Has Authority`
      (:`Authority`
        (`self.CustomRearm` self)))))

(event `SwitchRocket`
  (bind _sqvehicleinventory (`self.SQVehicleInventory`))
  (if (== (`SQPawnInventoryComponent.CurrentWeaponSlot` _sqvehicleinventory) 0)
    (`SQPawnInventoryComponent.SwitchWeapon` _sqvehicleinventory 1)
    (`SQEquipableItem.BeginUse` (`SQPawnInventoryComponent.CurrentWeapon` _sqvehicleinventory))
    (else
      (`SQPawnInventoryComponent.SwitchWeapon` _sqvehicleinventory 0))))

(event `self.ReceiveBeginPlay`
  (`parent.ReceiveBeginPlay`)
  (add `self.OnVehicleRepairEvent` (delegate `OnVehicleRepairEvent_Event_0`)))

(event `OnVehicleRepairEvent_Event_0` :!signature `self.OnVehicleRepairEvent`
  (params (Vehicle :type "SQVehicle Object Reference"))
  (`KismetSystemLibrary.Delay` 1.0)
  (`self.CustomRearm` Vehicle))

(event `CustomRearm`
  (params (NewParam :type "SQVehicle Object Reference"))
  (bind _returnvalue (`self.GetVehicleInventory` NewParam))
  (`/Engine/EditorBlueprintResources/StandardMacros.DoOnce` false :!label _label
    (:`Completed`
      (`KismetArrayLibrary.Array_Clear` (`SQPawnInventoryComponent.TestInventory` _returnvalue))
      (`KismetArrayLibrary.Array_Clear` (`SQVehicleInventoryComponent.Weapons` _returnvalue))
      (`SQPawnInventoryComponent.RemoveItemClassFromInventory` _returnvalue "/HelicopterTestMaps/Mi-8/BP_UB32_Mi8.BP_UB32_Mi8_C")
      (bind _returnvalue_2 (`SQPawnInventoryComponent.AddGroupToInventory` _returnvalue))
      (`SQPawnInventoryComponent.InsertItemIntoInventory` _returnvalue 0 (make `SQInventoryData` "/HelicopterTestMaps/Mi-8/BP_UB32_Mi8.BP_UB32_Mi8_C") _returnvalue_2)
      (bind _returnvalue_3 (`SQPawnInventoryComponent.AddGroupToInventory` _returnvalue))
      (`SQPawnInventoryComponent.InsertItemIntoInventory` _returnvalue 1 (make `SQInventoryData` "/HelicopterTestMaps/Mi-8/BP_UB32_Mi8_2.BP_UB32_Mi8_2_C") _returnvalue_3)
      (`KismetSystemLibrary.Delay` 5.0)
      (goto _label :!via `Reset`))))

(fn `UserConstructionScript`
  (`parent.UserConstructionScript`))