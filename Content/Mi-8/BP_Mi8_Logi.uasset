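; Logistics variant of the Mi-8 vehicle that shows its carried resources through static meshes.
; On non-authority instances, Tick retries until the first weapon in each of the first two inventory slots is valid.
; It casts each to SQVehicleResourceWeapon, assigns it a group of meshes and forces a visibility update.
; An Initialized flag ends the retries once both are set up.
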(event `self.ReceiveTick`
  (params (DeltaSeconds :type "Float (single-precision)"))
  (bind _testinventory (`SQPawnInventoryComponent.TestInventory` (`self.SQVehicleInventory`)))
  (bind _testinventory_2 (`SQPawnInventoryComponent.TestInventory` (`self.SQVehicleInventory`)))
  (bind _output_weapons (break `SQTestWeaponGroupData` (`|GetArrayItem` _testinventory 1)))
  (bind _output_weapons_2 (break `SQTestWeaponGroupData` (`|GetArrayItem` _testinventory_2)))
  (`parent.ReceiveTick` DeltaSeconds)
  (`/Engine/EditorBlueprintResources/ActorMacros.Switch Has Authority`
    (:`Remote`
      (if (`self.Initialized`)
        _
        (elif (`KismetArrayLibrary.Array_IsValidIndex` _testinventory_2)
          (if (`KismetArrayLibrary.Array_IsValidIndex` _output_weapons_2)
            (bind _assqvehicle_resource_weapon (cast `SQVehicleResourceWeapon` (`|GetArrayItem` _output_weapons_2)))
            (set `SQVehicleResourceWeapon.StaticMeshResources` (`|MakeArray` (`self.StaticMesh1`) (`self.StaticMesh2`) (`self.StaticMesh5`) (`self.StaticMesh6`) (`self.StaticMesh7`) (`self.StaticMesh8`) (`self.StaticMesh9`)) _assqvehicle_resource_weapon)
            (`SQVehicleResourceWeapon.ForceUpdateVisibilities` _assqvehicle_resource_weapon)
            (if (`KismetArrayLibrary.Array_IsValidIndex` _testinventory 1)
              (if (`KismetArrayLibrary.Array_IsValidIndex` _output_weapons)
                (bind _assqvehicle_resource_weapon_2 (cast `SQVehicleResourceWeapon` (`|GetArrayItem` _output_weapons)))
                (set `SQVehicleResourceWeapon.StaticMeshResources` (`|MakeArray` (`self.StaticMesh`) (`self.StaticMesh3`) (`self.StaticMesh4`)) _assqvehicle_resource_weapon_2)
                (`SQVehicleResourceWeapon.ForceUpdateVisibilities` _assqvehicle_resource_weapon_2)
                (set `self.Initialized` true)))))))))

(fn `UserConstructionScript`
  (`parent.UserConstructionScript`))