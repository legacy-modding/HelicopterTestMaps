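; Rocket launcher actor for the Mi-8 that fires S-5 rockets from a Firespot with launch sound and muzzle flash.
; FireRocketReload spawns a rocket if loaded, starts a timed reload and returns whether it fired.
; It also sets skeletal mesh physics velocity from the rocket's plus the parent actor's velocity, printing the latter.
; A separate SpawnRocket event fires an RPG-26 rocket without ammo checks.
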(event `self.ReceiveBeginPlay`)

(event `self.ReceiveTick`
  (params (DeltaSeconds :type "Float (single-precision)")))

(event `Spawn Rocket`
  (bind _firespot (`self.Firespot`))
  (bind _returnvalue (`SceneComponent.K2_GetComponentLocation` _firespot))
  (`|SpawnActorFromClass` "/Game/Blueprints/Items/Projectiles/Rockets/BP_RPG26_Rocket.BP_RPG26_Rocket_C" (`SceneComponent.K2_GetComponentToWorld` _firespot) "Undefined" "OverrideRootScale")
  (`GameplayStatics.PlaySoundAtLocation` "/Game/Vehicles/Technical/Weapons/UB-32/Sounds/Fire/3p/FFAR_fire_3p_Cue.FFAR_fire_3p_Cue" _returnvalue)
  (`GameplayStatics.SpawnEmitterAtLocation` "/Game/Particles/Weapons/Anti-Tank/Muzzleflash_S5.Muzzleflash_S5" _returnvalue (struct :`Pitch` -90.0)))

(fn `FireRocketReload`
  (returns (FiredRocket :type Boolean))
  (bind _firespot (`self.Firespot`))
  (bind _returnvalue (`SceneComponent.K2_GetComponentLocation` _firespot))
  (bind _returnvalue_2 (`self.GetVelocity` (`self.GetParentActor`)))
  (if (`self.HasAmmo`)
    (bind _returnvalue_3 (`|SpawnActorFromClass` "/Game/Blueprints/Items/Projectiles/Rockets/BP_S5.BP_S5_C" (`SceneComponent.K2_GetComponentToWorld` _firespot) "Undefined" "OverrideRootScale"))
    (`KismetSystemLibrary.PrintString` (`KismetStringLibrary.Conv_VectorToString` _returnvalue_2))
    (`PrimitiveComponent.SetAllPhysicsLinearVelocity` (`self.SkeletalMesh`) (+ (`self.GetVelocity` _returnvalue_3) _returnvalue_2) false)
    (`GameplayStatics.PlaySoundAtLocation` "/Game/Vehicles/Technical/Weapons/UB-32/Sounds/Fire/3p/FFAR_fire_3p_Cue.FFAR_fire_3p_Cue" _returnvalue)
    (`GameplayStatics.SpawnEmitterAtLocation` "/Game/Particles/Weapons/Anti-Tank/Muzzleflash_S5.Muzzleflash_S5" _returnvalue (struct :`Pitch` -90.0))
    (set `self.HasAmmo` false)
    (`KismetSystemLibrary.K2_SetTimer` null "ReloadRocket" (`self.ReloadTime`))
    (return true)
    (else
      (return false))))

(fn `ReloadRocket`
  (set `self.HasAmmo` true))

(fn `UserConstructionScript`)